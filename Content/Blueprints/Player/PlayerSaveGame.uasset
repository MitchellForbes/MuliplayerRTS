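; PlayerSaveGame stores the player's quest log and per-quest progress so it can be restored into the game instance.
; SaveQuestLog copies the active and completed quest lists, while SaveQuestDetails records each quest's stage and objective progress in a map keyed by quest ID.
; LoadQuests re-creates active quests through the game instance's AddNewQuest, applies their saved stage and progress, then overwrites its active and completed lists.
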(fn SaveQuestDetails
  (params (QuestBase :type Quest%20Base%20Object%20Reference))
  (Utilities|Map|Add (Variables|Default|GetQuestProgress) (Variables|/Game/QuestSystem/Blueprints/Quest_Base.Quest_Base_C|GetQuestID QuestBase) (Utilities|Struct|MakeStruct_FSaveQuestData (Variables|/Game/QuestSystem/Blueprints/Quest_Base.Quest_Base_C|GetCurrentObjectiveProgress QuestBase) (Variables|/Game/QuestSystem/Blueprints/Quest_Base.Quest_Base_C|GetCurrentStage QuestBase))))

(fn LoadQuests
  (params (GameInstance :type BP%20Artemis%20Frontier%20Game%20Instance%20Object%20Reference))
  (for _array_element (Variables|Default|GetCurrentActiveQuests)
    (bind _returnvalue (Default|AddNewQuest GameInstance _array_element))
    (Variables|/Game/QuestSystem/Blueprints/Quest_Base.Quest_Base_C|SetCurrentStage _returnvalue (.CurrentStage (Utilities|Struct|BreakStruct_FSaveQuestData (.Value (Utilities|Map|Find (Variables|Default|GetQuestProgress) _array_element)))))
    (Variables|/Game/QuestSystem/Blueprints/Quest_Base.Quest_Base_C|SetCurrentObjectiveProgress _returnvalue (.Progress (Utilities|Struct|BreakStruct_FSaveQuestData (.Value (Utilities|Map|Find (Variables|Default|GetQuestProgress) _array_element))))))
  (Variables|/Game/Blueprints/BP_ArtemisFrontierGameInstance.BP_ArtemisFrontierGameInstance_C|SetCurrentActiveQuests GameInstance (Variables|Default|GetCurrentActiveQuests))
  (Variables|/Game/Blueprints/BP_ArtemisFrontierGameInstance.BP_ArtemisFrontierGameInstance_C|SetCompletedQuests GameInstance (Variables|Default|GetCompletedQuests)))

(fn SaveQuestLog
  (params (NewParam :type BP%20Artemis%20Frontier%20Game%20Instance%20Object%20Reference))
  (Variables|Default|SetCurrentActiveQuests (Variables|/Game/Blueprints/BP_ArtemisFrontierGameInstance.BP_ArtemisFrontierGameInstance_C|GetCurrentActiveQuests NewParam))
  (Variables|Default|SetCompletedQuests (Variables|/Game/Blueprints/BP_ArtemisFrontierGameInstance.BP_ArtemisFrontierGameInstance_C|GetCompletedQuests NewParam)))