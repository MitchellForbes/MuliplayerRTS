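; RTS HUD that draws a translucent cyan drag-selection box on screen.
; StartSelection stores the mouse position as the first corner and turns drawing on; StopSelection turns it off.
; While drawing, DrawHUD reads the current mouse position each frame and draws a rectangle between the two corners.
; It only renders the box and does not select any actors.
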(event EventStartSelection
  (bind _returnvalue (Game|GetPlayerController 0))
  (bind (_locationx _locationy) (Game|Player|GetMousePosition _returnvalue))
  (Variables|Default|SetPointA (Math|Vector2D|MakeVector2D _locationx _locationy))
  (Variables|Default|SetIsDrawing true))

(event EventStopSelection
  (Variables|Default|SetIsDrawing false))

(event EventDrawHUD
  (params (SizeX :type Integer) (SizeY :type Integer))
  (bind _returnvalue (Game|GetPlayerController 0))
  (bind _pointa (Variables|Default|GetPointA))
  (bind (_locationx _locationy) (Game|Player|GetMousePosition _returnvalue))
  (if (Variables|Default|GetIsDrawing)
    (Variables|Default|SetPointB (Math|Vector2D|MakeVector2D _locationx _locationy))
    (HUD|DrawRect "(R=0.099210,G=0.852053,B=1.000000,A=0.500000)" (.x _pointa) (.y _pointa) (- (.x (Variables|Default|GetPointB)) (.x _pointa)) (- (.y (Variables|Default|GetPointB)) (.y _pointa)))))

(fn ConstructionScript)