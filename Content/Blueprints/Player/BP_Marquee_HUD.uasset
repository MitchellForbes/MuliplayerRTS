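; HUD Blueprint that provides drag-box selection of units derived from BP_ParentUnitClass.
; Marquee press, hold and release events track the mouse corners and drawing state, while DrawHUD paints a translucent green rectangle.
; During the drag, it selects units inside, clears the player controller's building selection, and deselects units outside, removing them from the array while looping over it.
; GetSelectedUnits exposes the resulting array.
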(event EventMarqueePressed
  (bind _returnvalue (Game|GetPlayerController 0))
  (bind (_locationx _locationy) (Game|Player|GetMousePosition _returnvalue))
  ;[1 1 1] Marquee Pressed
  (Variables|Default|SetIsDrawing? true)
  (bind _output_get (Variables|Default|SetStartMousePosition (Math|Vector2D|MakeVector2D _locationx _locationy)))
  (Variables|Default|SetCurrentMousePosition _output_get))

(event EventMarqueeHeld
  (bind _returnvalue (Game|GetPlayerController 0))
  (bind (_locationx _locationy) (Game|Player|GetMousePosition _returnvalue))
  ;[1 1 1] Marquee Held
  (Variables|Default|SetCurrentMousePosition (Math|Vector2D|MakeVector2D _locationx _locationy)))

(event EventMarqueeReleased
  ;[1 1 1] Marque Released
  (Variables|Default|SetIsDrawing? false))

(event EventDrawHUD
  (params (SizeX :type Integer) (SizeY :type Integer))
  (bind _startmouseposition (Variables|Default|GetStartMousePosition))
  (bind _currentmouseposition (Variables|Default|GetCurrentMousePosition))
  ;[1 1 1] Draw Marquee
  (if (Variables|Default|GetIsDrawing?)
    (HUD|DrawRect "(R=0.000000,G=1.000000,B=0.052163,A=0.200000)" (.x _startmouseposition) (.y _startmouseposition) (- (.x _currentmouseposition) (.x _startmouseposition)) (- (.y _currentmouseposition) (.y _startmouseposition)))
    (bind _output_get (Variables|Default|SetActorInDraw (Class|HUD|GetActorsinSelectionRectangle "/Game/Blueprints/Units/BP_ParentUnitClass.BP_ParentUnitClass_C" (Variables|Default|GetStartMousePosition) (Variables|Default|GetCurrentMousePosition) false false)))
    (for _array_element _output_get
      ;[1 1 1] Add Units To array
      (Class|BPIInterface|SelectThis(Message) _array_element)
      (Utilities|Array|AddUnique (Variables|Default|GetSelectedUnits) _array_element)
      (Class|BPIInterface|ClearSelectedBuilding(Message) (Game|GetPlayerController 0)))
    ;[1 1 1] Select only units in the Draw area
    (for _array_element_2 (Variables|Default|GetSelectedUnits)
      (if (== (Utilities|Array|FindItem (Variables|Default|GetActorInDraw) _array_element_2) -1)
        (Class|BPIInterface|DeselectThis(Message) _array_element_2)
        (Utilities|Array|RemoveItem (Variables|Default|GetSelectedUnits) _array_element_2)))))

(fn ConstructionScript)

(fn GetSelectedUnits
  (return (Variables|Default|GetSelectedUnits)))