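; BP_RTSCamera is the player's RTS camera actor, providing screen-edge scrolling and owning the resource count HUD.
; MouseX and MouseY events compare cursor position to viewport size and apply delta-time-scaled world offsets in the outer 2% margins.
; BeginPlay zeroes rotation and adds a W_ResourceCount widget for team 0.
; ToggleUI flip-flops that widget's visibility, starting with Visible, so the first press shows no change.
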(event EventBeginPlay
  (Utilities|FlowControl|Sequence
    (:then_0
      (Transformation|SetActorRotation "0, 0, 0")
      (bind _returnvalue (UserInterface|CreateWidget "/Game/UI/W_ResourceCount.W_ResourceCount_C" (Game|GetPlayerController 0)))
      (bind _output_get (Variables|Default|SetResourceCounter _returnvalue))
      (UserInterface|Viewport|AddtoViewport _output_get 0))))

(event Input|ActionEvents|InputActionToggleUI
  (params (Key :type Key%20Structure :default "None"))
  (:Pressed
    (Utilities|FlowControl|FlipFlop
      (:A
        (Widget|SetVisibility (Variables|Default|GetResourceCounter) "Visible"))
      (:B
        (Widget|SetVisibility (Variables|Default|GetResourceCounter) "Hidden")))))

(event Input|MouseEvents|MouseY
  (params (AxisValue :type Float%20%28single-precision%29))
  (bind _returnvalue (Game|GetPlayerController 0))
  (bind _returnvalue_2 (Viewport|GetViewportSize))
  (bind _returnvalue_3 (Utilities|Time|GetWorldDeltaSeconds))
  (bind _scrollspeed (Variables|Default|GetScrollSpeed))
  (bind _locationy (Game|Player|GetMousePosition _returnvalue))
  (bind _returnvalue_4 (* _scrollspeed _returnvalue_3))
  (bind _returnvalue_5 (/ _locationy (.y _returnvalue_2)))
  ;[1 1 1] edge Scrolling
  (if (> _returnvalue_5 0.98)
    (Transformation|AddActorWorldOffset (Math|Vector|MakeVector (* _returnvalue_4 -1.0) 0.0 0.0))
    (elif (< _returnvalue_5 0.02)
      (Transformation|AddActorWorldOffset (Math|Vector|MakeVector _returnvalue_4 0.0 0.0)))))

(event Input|MouseEvents|MouseX
  (params (AxisValue :type Float%20%28single-precision%29))
  (bind _returnvalue (Utilities|Time|GetWorldDeltaSeconds))
  (bind _returnvalue_2 (Game|GetPlayerController 0))
  (bind _returnvalue_3 (Viewport|GetViewportSize))
  (bind _scrollspeed (Variables|Default|GetScrollSpeed))
  (bind _locationx (Game|Player|GetMousePosition _returnvalue_2))
  (bind _returnvalue_4 (* _scrollspeed _returnvalue))
  (bind _returnvalue_5 (/ _locationx (.x _returnvalue_3)))
  ;[1 1 1] edge Scrolling
  (if (> _returnvalue_5 0.98)
    (Transformation|AddActorWorldOffset (Math|Vector|MakeVector 0.0 _returnvalue_4 0.0))
    (elif (< _returnvalue_5 0.02)
      (Transformation|AddActorWorldOffset (Math|Vector|MakeVector 0.0 (* _returnvalue_4 -1.0) 0.0)))))

(fn ConstructionScript)