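; Base RTS building actor that supports selection, team identity and a team-coloured mesh.
; On BeginPlay it applies a dynamic material instance carrying its team colour, and select and deselect events toggle a decal's visibility.
; Overlaps on the server send a DropoffMessage to the other actor.
; GetTeam returns the team number, while the resource increment, selected-units and team-check functions are placeholder stubs.
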(event EventBeginPlay
  (Utilities|FlowControl|Sequence
    (:then_0
      ;[1 1 1] Team Colour
      (bind _returnvalue (Rendering|Material|CreateDynamicMaterialInstance (Rendering|Material|GetMaterial (Variables|Default|GetBuildingMesh) 0) "None" "None" :!class /Script/Engine.KismetMaterialLibrary))
      (Rendering|Material|SetVectorParameterValue _returnvalue "TeamColour" (Variables|Default|GetTeamColour) :!class /Script/Engine.MaterialInstanceDynamic)
      (Rendering|Material|SetMaterial (Variables|Default|GetBuildingMesh) 0 _returnvalue))))

(event Collision|EventActorBeginOverlap
  (params (OtherActor :type Actor%20Object%20Reference))
  (Networking|SwitchHasAuthority
    (:Authority
      (Class|BPIResources|Dropoff(Message) OtherActor))))

(event EventSelectThis
  (Rendering|SetVisibility (Variables|Default|GetSelectedDecal) true false))

(event EventDeselectThis
  (Rendering|SetVisibility (Variables|Default|GetSelectedDecal) false false))

(fn ConstructionScript)

(fn GetSelectedUnits
  (return 0))

(fn GetTeam
  (return (Variables|Default|GetTeamNumber)))

(fn IncremenetWoodAmount
  (return 0))

(fn IncrementFoodAmount
  (return 0))

(fn IncrementMineralAmount
  (return 0))

(fn IsonMyTeam?
  (params (TeamNumber :type Integer))
  (return false))