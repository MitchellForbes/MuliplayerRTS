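; BP_HubDoor is a hinged door that swings open when something overlaps its DoorOpen component and closes when the overlap ends.
; BeginPlay caches the Pivot's relative rotation as closed and derives the open rotation by adding a 90-degree yaw.
; The Open timeline plays or reverses on overlap, interpolating the Pivot between both rotations through its DoorOpen track, with no filter on the overlapping actor.
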(event OnComponentBeginOverlap(DoorOpen)
  (params (OverlappedComponent :type Primitive%20Component%20Object%20Reference) (OtherActor :type Actor%20Object%20Reference) (OtherComp :type Primitive%20Component%20Object%20Reference) (OtherBodyIndex :type Integer) (bFromSweep :type Boolean) (SweepResult :type Hit%20Result%20Structure%20%28by%20ref%29))
  (bind _dooropen (Timeline|Open Play)
    (:Update
      (Transformation|SetRelativeRotation (Variables|Default|GetPivot) (Math|Rotator|Lerp(Rotator) (Variables|Default|GetClosedRotation) (Variables|Default|GetOpenRotation) (Math|Float|Lerp _dooropen 0.0 0.0)) false false))))

(event OnComponentEndOverlap(DoorOpen)
  (params (OverlappedComponent :type Primitive%20Component%20Object%20Reference) (OtherActor :type Actor%20Object%20Reference) (OtherComp :type Primitive%20Component%20Object%20Reference) (OtherBodyIndex :type Integer))
  (bind _dooropen (Timeline|Open Reverse)
    (:Update
      (Transformation|SetRelativeRotation (Variables|Default|GetPivot) (Math|Rotator|Lerp(Rotator) (Variables|Default|GetClosedRotation) (Variables|Default|GetOpenRotation) (Math|Float|Lerp _dooropen 0.0 0.0)) false false))))

(event EventBeginPlay
  (bind _output_get (Variables|Default|SetClosedRotation (Variables|/Script/Engine.SceneComponent|GetRelativeRotation (Variables|Default|GetPivot))))
  (Variables|Default|SetOpenRotation (Math|Rotator|CombineRotators _output_get (Math|Rotator|MakeRotator 0.0 0.0 9e+01))))

(fn ConstructionScript)