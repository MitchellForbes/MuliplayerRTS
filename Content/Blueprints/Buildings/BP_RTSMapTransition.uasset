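; BP_RTSMapTransition is a barrier actor that moves the player to the MapPrototype level once quest MQ001 is completed.
; Overlap by BP_ThirdPersonCharacter toggles actor input, a text prompt and a gate that lets IA_Interact through only inside the barrier.
; On a valid interact, it saves quest details through the game instance, creates a level sequence player without playing it, and opens the level.
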(event OnComponentBeginOverlap(Barrier)
  (params (OverlappedComponent :type Primitive%20Component%20Object%20Reference) (OtherActor :type Actor%20Object%20Reference) (OtherComp :type Primitive%20Component%20Object%20Reference) (OtherBodyIndex :type Integer) (bFromSweep :type Boolean) (SweepResult :type Hit%20Result%20Structure%20%28by%20ref%29))
  (Utilities|Casting|CastToBP_ThirdPersonCharacter OtherActor)
  (Input|EnableInput (Game|GetPlayerController 0))
  (Rendering|SetVisibility (Variables|Default|GetTextRender) true false)
  (Utilities|FlowControl|Gate true) ; enters at Open
)

(event OnComponentEndOverlap(Barrier)
  (params (OverlappedComponent :type Primitive%20Component%20Object%20Reference) (OtherActor :type Actor%20Object%20Reference) (OtherComp :type Primitive%20Component%20Object%20Reference) (OtherBodyIndex :type Integer))
  (Utilities|Casting|CastToBP_ThirdPersonCharacter OtherActor)
  (Input|DisableInput (Game|GetPlayerController 0))
  (Rendering|SetVisibility (Variables|Default|GetTextRender) false false)
  (Utilities|FlowControl|Gate true) ; enters at Close
)

(event Input|EnhancedActionEvents|EnhancedInputActionIA_Interact
  (params (ActionValue :type Boolean) (ElapsedSeconds :type Float%20%28double-precision%29) (TriggeredSeconds :type Float%20%28double-precision%29) (InputAction :type Input%20Action%20Object%20Reference :default "/Game/ThirdPerson/Input/Actions/IA_Interact.IA_Interact"))
  (bind _asbp_artemis_frontier_game_instance (Utilities|Casting|CastToBP_ArtemisFrontierGameInstance (Game|GetGameInstance)))
  (if (.ReturnValue (Default|QueryCompletedQuests _asbp_artemis_frontier_game_instance "MQ001"))
    (Utilities|FlowControl|Gate true
      (:Exit
        (bind _asbp_artemis_frontier_game_instance_2 (Utilities|Casting|CastToBP_ArtemisFrontierGameInstance (Game|GetGameInstance)))
        (Default|SaveQuestDetails _asbp_artemis_frontier_game_instance_2)
        (Sequencer|Player|CreateLevelSequencePlayer 0)
        (Game|OpenLevel(byObjectReference) "/Game/levels/MapPrototype.MapPrototype")))))

(fn ConstructionScript)