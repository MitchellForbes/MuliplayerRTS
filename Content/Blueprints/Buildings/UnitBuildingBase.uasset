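; Base RTS building that follows the cursor with a green placement material until clicked, then pays its resource cost or destroys itself.
; Left-clicking it once placed centers the camera and opens its build menu; overlapping actors get server-side dropoff messages.
; BuildUnit checks the building's own costs, then runs a timer shown on a camera-facing progress bar.
; SpawnUnit spawns near the rally point and only then deducts the unit's costs.
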(event Custom|PlaceBuilding
  (CallFunction|SetMeshMaterials)
  (Variables|Default|SetIsActive true)
  (bind _asbp_artemis_frontier_game_instance (Utilities|Casting|CastToBP_ArtemisFrontierGameInstance (Game|GetGameInstance)))
  (if (Math|Boolean|ANDBoolean (>= (Variables|/Game/Blueprints/BP_ArtemisFrontierGameInstance.BP_ArtemisFrontierGameInstance_C|GetResourceWood _asbp_artemis_frontier_game_instance) (Variables|Default|GetWoodCost)) (>= (Variables|/Game/Blueprints/BP_ArtemisFrontierGameInstance.BP_ArtemisFrontierGameInstance_C|GetResourceMinerals _asbp_artemis_frontier_game_instance) (Variables|Default|GetMineralCost)) (>= (Variables|/Game/Blueprints/BP_ArtemisFrontierGameInstance.BP_ArtemisFrontierGameInstance_C|GetResourceFood _asbp_artemis_frontier_game_instance) (Variables|Default|GetFoodCost)))
    (Class|BPIInterface|IncrementResourceAmount(Message) (Game|GetPlayerController 0) (* (Variables|Default|GetWoodCost) -1) "NewEnumerator0")
    (Class|BPIInterface|IncrementResourceAmount(Message) (Game|GetPlayerController 0) (* (Variables|Default|GetMineralCost) -1) "NewEnumerator1")
    (Class|BPIInterface|IncrementResourceAmount(Message) (Game|GetPlayerController 0) (* (Variables|Default|GetFoodCost) -1) "NewEnumerator2")
    (else
      (Actor|DestroyActor))))

(event Custom|BuildUnit
  (params (Unit%20Class :type BP%20Parent%20Unit%20Class%20Class%20Reference))
  (if (not (Utilities|Time|IsValidTimerHandle (Variables|Default|GetBuildTimer)))
    (bind _asbp_artemis_frontier_game_instance (Utilities|Casting|CastToBP_ArtemisFrontierGameInstance (Game|GetGameInstance)))
    (if (Math|Boolean|ANDBoolean (>= (Variables|/Game/Blueprints/BP_ArtemisFrontierGameInstance.BP_ArtemisFrontierGameInstance_C|GetResourceWood _asbp_artemis_frontier_game_instance) (Variables|Default|GetWoodCost)) (>= (Variables|/Game/Blueprints/BP_ArtemisFrontierGameInstance.BP_ArtemisFrontierGameInstance_C|GetResourceMinerals _asbp_artemis_frontier_game_instance) (Variables|Default|GetMineralCost)) (>= (Variables|/Game/Blueprints/BP_ArtemisFrontierGameInstance.BP_ArtemisFrontierGameInstance_C|GetResourceFood _asbp_artemis_frontier_game_instance) (Variables|Default|GetFoodCost)))
      (Variables|Default|SetCurrentBuildClass Unit%20Class)
      (bind _returnvalue (Utilities|Time|SetTimerbyEvent (delegate Custom|SpawnUnit) (Variables|Default|GetBuildTime)))
      (Variables|Default|SetBuildTimer _returnvalue)
      (Variables|Default|SetBuilding true))))

(event Custom|SpawnUnit
  (Variables|Default|SetBuilding false)
  (Rendering|SetVisibility (Variables|Default|GetProgressBar) false false)
  (bind _returnvalue (Game|SpawnActorfromClass (Variables|Default|GetCurrentBuildClass) (Math|Transform|MakeTransform (.RandomLocation (AI|Navigation|GetRandomReachablePointinRadius (Transformation|GetWorldLocation (Variables|Default|GetRallyPoint)) 1e+02 0 0))) "Undefined" "MultiplyWithRoot" 0 "(R=0.000000,G=0.000000,B=0.000000,A=0.000000)" 0 0))
  (Utilities|Time|ClearandInvalidateTimerbyHandle (Variables|Default|GetBuildTimer))
  (Utilities|IsValid _returnvalue
    (:Is%20Valid
      (Class|BPIInterface|IncrementResourceAmount(Message) (Game|GetPlayerController 0) (* (Variables|/Game/Blueprints/Units/BP_ParentUnitClass.BP_ParentUnitClass_C|GetWoodCost _returnvalue) -1) "NewEnumerator0")
      (Class|BPIInterface|IncrementResourceAmount(Message) (Game|GetPlayerController 0) (* (Variables|/Game/Blueprints/Units/BP_ParentUnitClass.BP_ParentUnitClass_C|GetMineralCost _returnvalue) -1) "NewEnumerator1")
      (Class|BPIInterface|IncrementResourceAmount(Message) (Game|GetPlayerController 0) (* (Variables|/Game/Blueprints/Units/BP_ParentUnitClass.BP_ParentUnitClass_C|GetFoodCost _returnvalue) -1) "NewEnumerator2"))))

(event EventBeginPlay
  (|CallParentFunction)
  (bind _returnvalue (Rendering|Material|CreateDynamicMaterialInstance 0 "None" "None" :!class /Script/Engine.KismetMaterialLibrary))
  (Variables|Default|SetFogOfWarMaterial _returnvalue)
  (bind _returnvalue_2 (Rendering|Material|CreateDynamicMaterialInstance 0 "None" "None" :!class /Script/Engine.KismetMaterialLibrary))
  (Variables|Default|SetFogOfWarRevealMaterial _returnvalue_2)
  (Variables|Default|SetMeshMaterials (Utilities|Array|MakeArray (Rendering|Material|GetMaterial (Variables|Default|GetBuildingMesh) 0) 0 0 0 0 0 0 0 0 0 0 0 0 0 0 0 0 0 0 0 0 0 0))
  (if (not (Variables|Default|GetIsActive))
    (CallFunction|SetGreenPlacement)))

(event EventTick
  (params (DeltaSeconds :type Float%20%28single-precision%29))
  (bind _returnvalue (Game|GetPlayerController 0))
  (bind (_hitresult _returnvalue_2) (Game|Player|GetHitResultUnderCursorbyChannel _returnvalue "TraceTypeQuery1" true))
  (if (not (Variables|Default|GetIsActive))
    (if _returnvalue_2
      (Transformation|SetActorLocation (.Location (Collision|BreakHitResult _hitresult)) false false))
    (elif (Variables|Default|GetBuilding)
      (CallFunction|OrinenttoCamera)
      (CallFunction|UnitProgress))))

(event Collision|EventActorBeginOverlap
  (params (OtherActor :type Actor%20Object%20Reference))
  (Networking|SwitchHasAuthority
    (:Authority
      (Class|BPIResources|Dropoff(Message) OtherActor))))

(event MouseInput|EventActorOnClicked
  (params (ButtonPressed :type Key%20Structure))
  (if (Variables|Default|GetIsActive)
    (if (== ButtonPressed "LeftMouseButton")
      (bind _aspc_rts (Utilities|Casting|CastToPC_RTS (Game|GetPlayerController 0)))
      (Default|ClearUnitSelection _aspc_rts)
      (|CallParentFunction ButtonPressed)
      (Default|SetCameraLocation (Variables|Default|GetAs%20RTS_Controller) (Transformation|GetActorLocation))
      (bind _returnvalue (UserInterface|CreateWidget "/Game/UI/BaseMenuUI.BaseMenuUI_C" 0 (Variables|Default|GetBuilding%20Menu%20Contents) self))
      (bind _output_get (Variables|Default|SetBaseMenu _returnvalue))
      (UserInterface|Viewport|AddtoViewport _output_get 0))
    (else
      (CallFunction|PlaceBuilding))))

(event EventIsSelected
  (params (IsSelected :type Boolean))
  (|CallParentFunction IsSelected)
  (if (not IsSelected)
    (Utilities|IsValid (Variables|Default|GetBaseMenu)
      (:Is%20Valid
        (Widget|RemovefromParent (Variables|Default|GetBaseMenu))
        (Variables|Default|SetBaseMenu 0)))))

(fn ConstructionScript
  (|CallParentFunction))

(fn SetGreenPlacement
  (for _index (range 0 (Utilities|Array|LastIndex (Variables|Default|GetMeshMaterials)))
    (Rendering|Material|SetMaterial (Variables|Default|GetBuildingMesh) _index "/Game/Blueprints/Buildings/Materials/GreenPlacement.GreenPlacement"))
  (Variables|Default|SetIsActive false))

(fn SetMeshMaterials
  (for (_array_element _array_index) (Variables|Default|GetMeshMaterials)
    (Rendering|Material|SetMaterial (Variables|Default|GetBuildingMesh) _array_index _array_element)))

(fn UnitProgress
  (bind _progressbar (Variables|Default|GetProgressBar))
  (bind _returnvalue (UserInterface|GetUserWidgetObject _progressbar))
  (bind _asprogress_bar (Utilities|Casting|CastToProgressBar _returnvalue))
  (Utilities|IsValid _asprogress_bar
    (:Is%20Valid
      (Progress|SetPercent (Variables|/Game/UI/ProgressBar.ProgressBar_C|GetProgressBar_19 _asprogress_bar) (/ (Class|KismetSystemLibrary|GetTimerElapsedTimeHandle (Variables|Default|GetBuildTimer)) (Variables|Default|GetBuildTime)))
      (Rendering|SetVisibility (Variables|Default|GetProgressBar) true false)
      (return))
    (:Is%20Not%20Valid
      (return))))

(fn SetRedPlacement
  (for _index (range 0 (Utilities|Array|LastIndex (Variables|Default|GetMeshMaterials)))
    (Rendering|Material|SetMaterial (Variables|Default|GetBuildingMesh) _index "/Game/Blueprints/Buildings/Materials/RedPlacement.RedPlacement"))
  (Variables|Default|SetIsActive false))

(fn OrinenttoCamera
  (bind _returnvalue (Game|GetPlayerCameraManager 0))
  (bind _progressbar (Variables|Default|GetProgressBar))
  (bind _progressbar_2 (Variables|Default|GetProgressBar))
  (bind _returnvalue_2 (Transformation|GetWorldLocation _progressbar))
  (bind _transformcomponent (Variables|/Script/Engine.PlayerCameraManager|GetTransformComponent _returnvalue))
  (bind _returnvalue_3 (Transformation|GetWorldLocation _transformcomponent))
  (bind _returnvalue_4 (Math|Rotator|FindLookatRotation _returnvalue_2 _returnvalue_3))
  (bind _returnvalue_5 (Math|Rotator|MakeRotator (.roll _returnvalue_4) (.pitch _returnvalue_4) (.yaw _returnvalue_4)))
  (Utilities|IsValid _progressbar_2
    (:Is%20Valid
      (Transformation|SetWorldRotation _progressbar_2 (Math|Rotator|MakeRotator (.roll _returnvalue_5) (.pitch _returnvalue_5) (.yaw _returnvalue_5)) false false)
      (return))))