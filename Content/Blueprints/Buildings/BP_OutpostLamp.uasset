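; BP_OutpostLamp is an outpost lamp that shows its Sphere component at night and hides it during the day.
; Each Tick it reads TimeofDay from the Artemis Frontier game instance and sets visibility on the Sphere and its children, treating after 18 or before 6 as night.
; Tick also adds a new audio component every frame, before the time check.
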(event EventBeginPlay)

(event Collision|EventActorBeginOverlap
  (params (OtherActor :type Actor%20Object%20Reference)))

(event EventTick
  (params (DeltaSeconds :type Float%20%28single-precision%29))
  (bind _asbp_artemis_frontier_game_instance (Utilities|Casting|CastToBP_ArtemisFrontierGameInstance (Game|GetGameInstance)))
  (AddComponent|AddAudioComponent false)
  (if (or (> (Variables|/Game/Blueprints/BP_ArtemisFrontierGameInstance.BP_ArtemisFrontierGameInstance_C|GetTimeofDay _asbp_artemis_frontier_game_instance) 18.0) (< (Variables|/Game/Blueprints/BP_ArtemisFrontierGameInstance.BP_ArtemisFrontierGameInstance_C|GetTimeofDay _asbp_artemis_frontier_game_instance) 6.0))
    (Rendering|SetVisibility (Variables|Default|GetSphere) true true)
    (else
      (Rendering|SetVisibility (Variables|Default|GetSphere) false true))))

(fn ConstructionScript)