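; E1 unit, apparently an enemy, that automatically damages worker units near it and can itself be killed.
; A box overlap adds Unit_Worker actors to UnitsInRange and starts a one-second timer; end overlap removes them.
; Each timer tick calls UnitDamaged on every listed BP_ParentUnitClass, re-arming itself while the first entry is valid.
; Its own UnitDamaged subtracts health and destroys it at zero; a montage-playing Attack function is not called here.
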(event OnComponentEndOverlap(Box)
  (params (OverlappedComponent :type Primitive%20Component%20Object%20Reference) (OtherActor :type Actor%20Object%20Reference) (OtherComp :type Primitive%20Component%20Object%20Reference) (OtherBodyIndex :type Integer))
  (Utilities|Array|RemoveItem (Variables|Default|GetUnitsInRange) OtherActor))

(event OnComponentBeginOverlap(Box)
  (params (OverlappedComponent :type Primitive%20Component%20Object%20Reference) (OtherActor :type Actor%20Object%20Reference) (OtherComp :type Primitive%20Component%20Object%20Reference) (OtherBodyIndex :type Integer) (bFromSweep :type Boolean) (SweepResult :type Hit%20Result%20Structure%20%28by%20ref%29))
  (Utilities|Casting|CastToUnit_Worker OtherActor)
  (Utilities|Array|AddUnique (Variables|Default|GetUnitsInRange) OtherActor)
  ;[1 1 1] Starts attack
  (CallFunction|AttackUnit))

(event Custom|AttackUnit
  ;[1 1 1] Current Damage Event
  (if (!= self (Utilities|Array|Get(acopy) (Variables|Default|GetUnitsInRange)))
    ;;[1 1 1] Attack Delay
    (Utilities|Time|SetTimerbyFunctionName 0 "DamageUnit" 1.0 true)))

(event Custom|DamageUnit
  ;[1 1 1] Current Damage Event
  (for _array_element (Variables|Default|GetUnitsInRange)
    (bind _asbp_parent_unit_class (Utilities|Casting|CastToBP_ParentUnitClass _array_element))
    (Utilities|IsValid _asbp_parent_unit_class
      (:Is%20Valid
        (Default|UnitDamaged _asbp_parent_unit_class (Variables|Default|GetDamage))
        (Utilities|IsValid (Utilities|Array|Get(acopy) (Variables|Default|GetUnitsInRange))
          (:Is%20Valid
            (Utilities|Time|SetTimerbyFunctionName 0 "DamageUnit" 1.0)))))))

(fn ConstructionScript)

(fn UnitDamaged
  (params (Damage :type Float%20%28double-precision%29))
  ;[1 1 1] Sets Damage
  (bind _output_get (LocalVariables|SetDamageLocal Damage))
  ;[1 1 1] Sets health
  (Variables|Default|SetCurrentHealth (- (Variables|Default|GetCurrentHealth) _output_get))
  ;[1 1 1] Is Unit Dead
  (if (<= (Variables|Default|GetCurrentHealth) 0.0)
    (Actor|DestroyActor))
  (return))

(fn Attack
  ;[1 1 1] Attack animation duration
  (Animation|PlayAnimMontage 0 1.0 "None")
  (return 0.0))