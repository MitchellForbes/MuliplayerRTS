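; BP_E2_Unit is an AI unit prototype that reacts to the player's Unit_Worker, cached on BeginPlay.
; WalkTowards, despite its name, moves to a random reachable point around a spot slightly away from the worker.
; BeginPlay and both move outcomes call RunAway, which is empty, and nothing here calls WalkTowards, so no movement loop runs.
; Box overlap with a worker only prints an attack debug message.
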(event OnComponentBeginOverlap(Box)
  (params (OverlappedComponent :type Primitive%20Component%20Object%20Reference) (OtherActor :type Actor%20Object%20Reference) (OtherComp :type Primitive%20Component%20Object%20Reference) (OtherBodyIndex :type Integer) (bFromSweep :type Boolean) (SweepResult :type Hit%20Result%20Structure%20%28by%20ref%29))
  (Utilities|Casting|CastToUnit_Worker OtherActor)
  (Development|PrintString "Attacking"))

(event Custom|WalkTowards
  (bind _returnvalue (Transformation|GetActorLocation))
  (bind _unit_ref (Variables|Default|GetUnit%20REF))
  (bind _returnvalue_2 (Transformation|GetActorLocation _unit_ref))
  (bind _returnvalue_3 (Math|Rotator|FindLookatRotation _returnvalue _returnvalue_2))
  (bind _returnvalue_4 (Math|Vector|GetForwardVector _returnvalue_3))
  (bind _returnvalue_5 (* _returnvalue_4 -5e+01))
  (bind _returnvalue_6 (+ _returnvalue _returnvalue_5))
  (bind (_x _y) (Math|Vector|BreakVector _returnvalue_6))
  (AI|AIMoveTo self (.RandomLocation (AI|Navigation|GetRandomReachablePointinRadius (Math|Vector|MakeVector _x _y (.Z (Math|Vector|BreakVector _returnvalue))) 1.5e+02 0 0)) 0 5.0 false
    (:OnSuccess
      _)
    (:OnFail
      _))
  (CallFunction|RunAway)
  (Development|PrintString "Tracking"))

(event EventBeginPlay
  (bind _asunit_worker (Utilities|Casting|CastToUnit_Worker (Game|GetPlayerCharacter 0)))
  (Variables|Default|SetUnit%20REF _asunit_worker)
  (CallFunction|RunAway))

(fn ConstructionScript)

(fn RunAway)