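; Base enemy AI class that roams around its spawn point, hunts player units and damages them in melee.
; Tick drops targets beyond DetectRange, scans all BP_ParentUnitClass actors for the first one in range, and chases it with AIMoveTo behind a resettable DoOnce.
; Units overlapping its Box take timer-driven damage.
; UnitDamage reduces its health, updating a camera-facing health bar that hides at full health, and destroys it at zero.
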(event OnComponentEndOverlap(Box)
  (params (OverlappedComponent :type Primitive%20Component%20Object%20Reference) (OtherActor :type Actor%20Object%20Reference) (OtherComp :type Primitive%20Component%20Object%20Reference) (OtherBodyIndex :type Integer))
  (Utilities|Array|RemoveItem (Variables|Default|GetUnits%20in%20Range) OtherActor))

(event OnComponentBeginOverlap(Box)
  (params (OverlappedComponent :type Primitive%20Component%20Object%20Reference) (OtherActor :type Actor%20Object%20Reference) (OtherComp :type Primitive%20Component%20Object%20Reference) (OtherBodyIndex :type Integer) (bFromSweep :type Boolean) (SweepResult :type Hit%20Result%20Structure%20%28by%20ref%29))
  (bind _asbp_parent_unit_class (Utilities|Casting|CastToBP_ParentUnitClass OtherActor))
  (Utilities|Array|AddUnique (Variables|Default|GetUnits%20in%20Range) _asbp_parent_unit_class)
  ;[1 1 1] Starts attack
  (CallFunction|AttackUnit))

(event Custom|AttackUnit
  ;[1 1 1] Current Damage Event
  (if (!= self (Utilities|Array|Get(acopy) (Variables|Default|GetUnits%20in%20Range)))
    ;;[1 1 1] Attack Delay
    (Utilities|Time|SetTimerbyFunctionName 0 "DamageUnit" 1.0 true)))

(event Custom|DamageUnit
  ;[1 1 1] Current Damage Event
  (for _array_element (Variables|Default|GetUnits%20in%20Range)
    (bind _asbp_parent_unit_class (Utilities|Casting|CastToBP_ParentUnitClass _array_element))
    (Utilities|IsValid _asbp_parent_unit_class
      (:Is%20Valid
        (Default|UnitDamaged _asbp_parent_unit_class (Variables|UnitCombat|GetDamage))
        (Utilities|IsValid (Utilities|Array|Get(acopy) (Variables|Default|GetUnits%20in%20Range))
          (:Is%20Valid
            (Utilities|Time|SetTimerbyFunctionName 0 "DamageUnit" 1.0)))))))

(event Custom|Roam
  (bind (_randomlocation _returnvalue) (Class|NavigationSystemV1|GetRandomLocationinNavigableRadius (Variables|Default|GetStartLocation) 1e+03 0 0))
  (if _returnvalue
    (AI|AIMoveTo self _randomlocation 0 5.0 false
      (:OnSuccess
        (Utilities|FlowControl|RetriggerableDelay (Math|Random|RandomFloatinRange 1.0 3.0))
        (CallFunction|Roam)))))

(event EventBeginPlay
  (Utilities|FlowControl|Sequence
    (:then_0
      (Variables|Default|SetStartLocation (Transformation|GetActorLocation))
      (bind _outactors (Actor|GetAllActorsOfClass "/Game/Blueprints/Units/BP_ParentUnitClass.BP_ParentUnitClass_C"))
      (Variables|Default|SetUnits _outactors))
    (:then_1
      (CallFunction|UpdateUnitHealthBar)
      (CallFunction|Roam))))

(event EventTick
  (params (DeltaSeconds :type Float%20%28single-precision%29))
  (bind _self self)
  (bind _unit (Variables|Default|GetUnit))
  (bind _unit_2 (Variables|Default|GetUnit))
  (bind _returnvalue (Transformation|GetActorLocation _unit))
  (bind _returnvalue_2 (Transformation|GetActorLocation _self))
  (bind _returnvalue_3 (Math|Rotator|FindLookatRotation _returnvalue_2 _returnvalue))
  (Utilities|FlowControl|Sequence
    (:then_0
      (CallFunction|ResetTarget)
      ;[1 1 1] Enemy Tracking - Finding & Reseting dection
      (Utilities|IsValid _unit_2
        (:Is%20Valid
          (Utilities|FlowControl|DoOnce false :!label _label
            (:Completed
              (AI|AIMoveTo (AI|GetAIController self) "0, 0, 0" _unit_2 4.0 "Default" "Default" true true
                (:then
                  ;[1 1 1] Enemy Facing Rotation
                  (Transformation|SetActorRotation (Math|Rotator|MakeRotator (.roll _returnvalue_3) 0.0 (.yaw _returnvalue_3))))
                (:OnRequestFailed
                  (goto _label Reset))
                (:OnMoveFinished
                  (goto _label Reset))))))
        (:Is%20Not%20Valid
          (CallFunction|FindNewTarget)
          (goto _label Reset))))
    (:then_1
      (CallFunction|OrientHealthtoCamera))))

(fn ConstructionScript)

(fn ResetTarget
  (if (>= (Transformation|GetDistanceTo (Variables|Default|GetUnit)) (Variables|Default|GetDetectRange))
    (Variables|Default|SetUnit 0)
    (Class|NavMovementComponent|StopActiveMovement (Variables|Character|GetCharacterMovement))
    (CallFunction|Roam))
  (return))

(fn FindNewTarget
  (bind _outactors (Actor|GetAllActorsOfClass "/Game/Blueprints/Units/BP_ParentUnitClass.BP_ParentUnitClass_C"))
  (Variables|Default|SetUnits _outactors)
  (for _array_element (Variables|Default|GetUnits)
    (Utilities|IsValid _array_element
      (:Is%20Valid
        (if (<= (Transformation|GetDistanceTo _array_element) (Variables|Default|GetDetectRange))
          (Variables|Default|SetUnit _array_element)
          (return))))))

(fn UnitDamage
  (params (Damage :type Float%20%28double-precision%29))
  ;[1 1 1] Sets Damage
  (bind _output_get (Variables|UnitCombat|SetDamage Damage))
  ;[1 1 1] Sets health
  (Variables|UnitCombat|SetCurrent%20Health (- (Variables|UnitCombat|GetCurrent%20Health) _output_get))
  ;[1 1 1] Is Unit Dead
  (if (<= (Variables|UnitCombat|GetCurrent%20Health) 0.0)
    (Actor|DestroyActor)
    (else
      (CallFunction|UpdateUnitHealthBar)))
  (return))

(fn OrientHealthtoCamera
  (bind _returnvalue (Game|GetPlayerCameraManager 0))
  (bind _enemyhealthbar (Variables|Default|GetEnemyHealthBar))
  (bind _enemyhealthbar_2 (Variables|Default|GetEnemyHealthBar))
  (bind _returnvalue_2 (Transformation|GetWorldLocation _enemyhealthbar))
  (bind _transformcomponent (Variables|/Script/Engine.PlayerCameraManager|GetTransformComponent _returnvalue))
  (bind _returnvalue_3 (Transformation|GetWorldLocation _transformcomponent))
  (bind _returnvalue_4 (Math|Rotator|FindLookatRotation _returnvalue_2 _returnvalue_3))
  (Utilities|IsValid _enemyhealthbar_2
    (:Is%20Valid
      (Transformation|SetWorldRotation _enemyhealthbar_2 (Math|Rotator|MakeRotator (.roll _returnvalue_4) (.pitch _returnvalue_4) (.yaw _returnvalue_4)) false false)
      (return))))

(fn UpdateUnitHealthBar
  (bind _maxhealth (Variables|UnitCombat|GetMaxHealth))
  (bind _current_health (Variables|UnitCombat|GetCurrent%20Health))
  (bind _returnvalue (/ _current_health _maxhealth))
  (Progress|SetPercent (Variables|/Game/Blueprints/Units/WB_UnitHealthBar.WB_UnitHealthBar_C|GetHealthProgBar (.AsWB%20Unit%20Health%20Bar (Utilities|Casting|CastToWB_UnitHealthBar (UserInterface|GetUserWidgetObject (Variables|Default|GetEnemyHealthBar))))) _returnvalue)
  (if (== _returnvalue 1.0)
    (Rendering|SetVisibility (Variables|Default|GetEnemyHealthBar) false false)
    (else
      (Rendering|SetVisibility (Variables|Default|GetEnemyHealthBar) true false)))
  (return))