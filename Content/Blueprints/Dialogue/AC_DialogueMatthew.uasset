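; Dialogue component that runs Commander Vanguarre's mission briefing to Arcas, sending the player to help Captain Acosta organise resources at Colony Atalanta.
; It overrides the parent Dialogue function and switches on DialogueTreeIndex, with only tree 0 defined.
; Chained AddDialogue calls branch on the chosen reply, with a casual greeting earning a rebuke before both paths converge on the briefing.
; The final reply calls RemoveDialogueProgress and closes the conversation.
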(fn Dialogue
  (|CallParentFunction)
  (switch int (Variables|Default|GetDialogueTreeIndex)
    (:0
      (bind (_state _optionindex) (CallFunction|AddDialogue "Commander Vanguarre" "Howzit, Arcas?" (Utilities|Array|MakeArray "Hi, Commander!" "What's up, Commander?")))
      (switch Utilities|FlowControl|Switch|SwitchonEnum_DialogueState _state
        (:NewEnumerator0
          (switch int _optionindex
            (:0
              (bind (_state_2 _optionindex_2) (CallFunction|AddDialogue "Commander Vanguarre" "I've got a mission for you." (Utilities|Array|MakeArray "What is it, sir?")))
              (switch Utilities|FlowControl|Switch|SwitchonEnum_DialogueState _state_2
                (:NewEnumerator0
                  (switch int _optionindex_2
                    (:0
                      _)))))
            (:1
              (bind (_state_3 _optionindex_3) (CallFunction|AddDialogue "Commander Vanguarre" "A little more respect next time, lad. Now, I have a mission for you." (Utilities|Array|MakeArray "Sorry, sir. What's the mission?")))
              (switch Utilities|FlowControl|Switch|SwitchonEnum_DialogueState _state_3
                (:NewEnumerator0
                  (switch int _optionindex_3
                    (:0
                      _))))))
          (bind _state_4 (CallFunction|AddDialogue "Commander Vanguarre" "We've only had Colony Atalanta up and running for a couple months now. Certain departments are in need of some help in organising resources. Check in with Captain Acosta to see what she needs." (Utilities|Array|MakeArray "Will do, sir. I'm looking forward to getting our new home working!")))
          (switch Utilities|FlowControl|Switch|SwitchonEnum_DialogueState _state_4
            (:NewEnumerator0
              (CallFunction|RemoveDialogueProgress 3)
              (CallFunction|CloseConversation))))))))