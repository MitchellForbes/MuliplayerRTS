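; Dialogue component that scripts Captain Acosta's briefing to Arcas about mining local minerals for Colony Atalanta.
; The Dialogue override calls its parent, then switches on DialogueTreeIndex, with only tree 0 defined.
; That tree is a linear chain of four nested AddDialogue calls, each offering one player reply and advancing on the Pass Through state.
; The last reply calls RemoveDialogueProgress and closes the conversation.
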(fn Dialogue
  (|CallParentFunction)
  (switch int (Variables|Default|GetDialogueTreeIndex)
    (:0
      (bind (_state _optionindex) (CallFunction|AddDialogue "Captain Acosta" "Hello, Arcas. Good to see you." (Utilities|Array|MakeArray "You too, Captain. I heard you could use some help?")))
      (switch Utilities|FlowControl|Switch|SwitchonEnum_DialogueState _state
        (:NewEnumerator0
          (switch int _optionindex
            (:0
              (bind (_state_2 _optionindex_2) (CallFunction|AddDialogue "Captain Acosta" "Indeed. We're slated to receive more colonists in the next few months, so we need to make sure we have enough industry up and running." (Utilities|Array|MakeArray "Of course. What do we need?")))
              (switch Utilities|FlowControl|Switch|SwitchonEnum_DialogueState _state_2
                (:NewEnumerator0
                  (switch int _optionindex_2
                    (:0
                      (bind (_state_3 _optionindex_3) (CallFunction|AddDialogue "Captain Acosta" "I want you to assist with mining 500 of the local minerals. We set Colony Atalanta up near to some to the WEST, so we can get started quickly." (Utilities|Array|MakeArray "Absolutely. Where do I go to begin?")))
                      (switch Utilities|FlowControl|Switch|SwitchonEnum_DialogueState _state_3
                        (:NewEnumerator0
                          (switch int _optionindex_3
                            (:0
                              (bind (_state_4 _optionindex_4) (CallFunction|AddDialogue "Captain Acosta" "If you head back into the main building, there's a console where you can communicate with the mining corps. Now get on with it, the busy madness never stops when you're building Earth 2.0!" (Utilities|Array|MakeArray "Heh, I'm beginning to get that impression...")))
                              (switch Utilities|FlowControl|Switch|SwitchonEnum_DialogueState _state_4
                                (:NewEnumerator0
                                  (CallFunction|RemoveDialogueProgress _optionindex_4)
                                  (CallFunction|CloseConversation))))))))))))))))))