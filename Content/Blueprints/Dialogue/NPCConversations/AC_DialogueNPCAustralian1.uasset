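; Dialogue component for an Australian Artemisian colonist NPC, giving a short monologue about missing Sydney and settling on Artemis.
; It overrides Dialogue, calls the parent, then switches on DialogueTreeIndex, with only tree 0 defined.
; Two chained AddDialogue nodes show the lines with Continue and Close options, branching on returned state and option index.
; The final option removes dialogue progress and closes the conversation.
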(fn Dialogue
  (|CallParentFunction)
  (switch int (Variables|Default|GetDialogueTreeIndex)
    (:0
      (bind (_state _optionindex) (CallFunction|AddDialogue "Aus. Artemisian Colonist" "I used to miss Sydney pretty bad... But after living on Artemis for two years, this has become my home." (Utilities|Array|MakeArray "Continue")))
      (switch Utilities|FlowControl|Switch|SwitchonEnum_DialogueState _state
        (:NewEnumerator0
          (switch int _optionindex
            (:0
              (bind _state_2 (CallFunction|AddDialogue "Aus. Artemisian Colonist" "Maybe I can ask Scout Lieutenant Noah to keep an eye out for any pathways to the ocean...?" (Utilities|Array|MakeArray "Close")))
              (switch Utilities|FlowControl|Switch|SwitchonEnum_DialogueState _state_2
                (:NewEnumerator0
                  (CallFunction|RemoveDialogueProgress 2)
                  (CallFunction|CloseConversation))))))))))