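; AC_DialogueNPCUS1 is an NPC conversation Blueprint giving a US Artemisian Colonist a short flavour dialogue about Ethel and two years on Artemis.
; Its Dialogue function calls the parent, then switches on the dialogue tree index, with only tree 0 defined.
; That tree chains two single-option lines; choosing Close on the second removes dialogue progress and closes the conversation.
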(fn Dialogue
  (|CallParentFunction)
  (switch int (Variables|Default|GetDialogueTreeIndex)
    (:0
      (bind (_state _optionindex) (CallFunction|AddDialogue "US Artemisian Colonist" "Two years on Artemis now... Wonder if Ethel will organise a get together...?" (Utilities|Array|MakeArray "Continue")))
      (switch Utilities|FlowControl|Switch|SwitchonEnum_DialogueState _state
        (:NewEnumerator0
          (switch int _optionindex
            (:0
              (bind _state_2 (CallFunction|AddDialogue "US Artemisian Colonist" "Who knows what weird incense she's found from the Fields?" (Utilities|Array|MakeArray "Close")))
              (switch Utilities|FlowControl|Switch|SwitchonEnum_DialogueState _state_2
                (:NewEnumerator0
                  (CallFunction|RemoveDialogueProgress 2)
                  (CallFunction|CloseConversation))))))))))