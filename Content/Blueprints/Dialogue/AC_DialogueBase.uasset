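; Base dialogue component that runs an NPC's branching conversation through a W_Dialogue widget, halting wandering NPCs and setting their IsInDialogue blackboard flag.
; The empty Dialogue function is replayed from the start after each choice: AddDialogue returns saved options by index and displays the first unanswered line.
; Closing removes the widget, clears the flag, reports quest-giver objectives through the game instance and conditionally sends the owner a conversation-closed message.
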(fn OpenConversation
  (params (SelectDialogue :type Integer))
  (Variables|Default|SetDialogueTreeIndex SelectDialogue)
  (bind _asnpc_wandering_npc (Utilities|Casting|CastToNPC_WanderingNPC (Components|GetOwner))
    (:then
      (AI|Navigation|StopMovement (Pawn|GetController _asnpc_wandering_npc))
      (AI|Components|Blackboard|SetValueasBool (AI|GetBlackboard (Pawn|GetController _asnpc_wandering_npc)) (Variables|Default|GetIsInDialogue) true))
    (:CastFailed
      _))
  (bind _returnvalue (UserInterface|CreateWidget "/Game/Blueprints/Dialogue/Widgets/W_Dialogue.W_Dialogue_C" 0 self))
  (bind _output_get (Variables|Default|SetDialogueWidget _returnvalue))
  (UserInterface|Viewport|AddtoViewport _output_get 0)
  (CallFunction|ProgressDialogue))

(fn CloseConversation
  (bind _returnvalue (Components|GetOwner))
  (bind _returnvalue_2 (Actor|GetComponentbyClass _returnvalue "/Game/QuestSystem/Components/BPC_QuestGiver.BPC_QuestGiver_C"))
  (Widget|RemovefromParent (Variables|Default|GetDialogueWidget))
  (bind _asnpc_wandering_npc (Utilities|Casting|CastToNPC_WanderingNPC (Components|GetOwner))
    (:then
      (AI|Components|Blackboard|SetValueasBool (AI|GetBlackboard (Pawn|GetController _asnpc_wandering_npc)) (Variables|Default|GetIsInDialogue) false))
    (:CastFailed
      _))
  (Utilities|IsValid _returnvalue_2
    (:Is%20Valid
      (bind _newparam (Default|PreRecQuests _returnvalue_2))
      (if _newparam
        (bind _objectiveid (Class|IColonyInterface|Interactwith(Message) _returnvalue))
        (bind _asbp_artemis_frontier_game_instance (Utilities|Casting|CastToBP_ArtemisFrontierGameInstance (Game|GetGameInstance)))
        (Default|CallOnObjectiveIDCalled _asbp_artemis_frontier_game_instance _objectiveid 1)
        (bind _foundwidgets (Widget|GetAllWidgetsOfClass "/Game/QuestSystem/Widgets/W_QuestWindow.W_QuestWindow_C" true))
        (Utilities|IsValid (Utilities|Array|Get(acopy) _foundwidgets)
          (:Is%20Not%20Valid
            (Class|BPIInteractable|ConversationClosed(Message) (Components|GetOwner))))
        (else
          (Class|BPIInteractable|ConversationClosed(Message) _returnvalue :!label _label))))
    (:Is%20Not%20Valid
      (goto _label))))

(fn ProgressDialogue
  (Variables|Default|SetDialogueIndex -1)
  (CallFunction|Dialogue))

(fn Dialogue)

(fn AddDialogue
  (params (Speaker :type Text) (Dialogue :type Text) (OptionsText :type Array%20of%20Texts))
  (bind _dialogueprogress (Variables|Default|GetDialogueProgress))
  (bind _dialogueindex (Variables|Default|GetDialogueIndex))
  (bind (_value _returnvalue) (Utilities|Map|Find _dialogueprogress _dialogueindex))
  (Math|Integer|IncrementInt (Variables|Default|GetDialogueIndex)
    (:%20%20
      (if _returnvalue
        (return "NewEnumerator0" _value)
        (else
          (Default|UpdateDialogueText (Variables|Default|GetDialogueWidget) Speaker Dialogue OptionsText (Variables|Default|GetDialogueIndex))
          (return "NewEnumerator1" 0))))))

(fn UpdateSelectedOption
  (params (ProgressIndex :type Integer%20%28by%20ref%29) (OptionIndex :type Integer%20%28by%20ref%29))
  (Utilities|Map|Add (Variables|Default|GetDialogueProgress) ProgressIndex OptionIndex)
  (CallFunction|ProgressDialogue))

(fn ClearDialogueProgress
  (Utilities|Map|Clear (Variables|Default|GetDialogueProgress)))

(fn RemoveDialogueProgress
  (params (ProgressSteps :type Integer))
  (for _index (range 0 ProgressSteps)
    (Utilities|Map|Remove (Variables|Default|GetDialogueProgress) (- (Variables|Default|GetDialogueIndex) _index))))

(fn SetDialogueTreeIndex
  (params (DialogueTreeIndex :type Integer))
  (Variables|Default|SetDialogueTreeIndex DialogueTreeIndex)
  (CallFunction|ClearDialogueProgress))