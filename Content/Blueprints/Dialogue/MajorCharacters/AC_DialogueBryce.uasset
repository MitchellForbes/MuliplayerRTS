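; Dialogue component for Coordinator Bryce Damar, the militia NPC who introduces the MQ003 culling quest and RTS combat.
; Dialogue extends the parent and switches on DialogueTreeIndex between introduction, combat tutorial and post-mission check-in, each a chain of single-option AddDialogue stages with play-once voice cues.
; The tutorial pans NPC_BryceDamar's camera to points of interest.
; Branches end by closing the conversation; the latter two also remove W_Dialogue widgets.
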(event Custom|Delay
  (Utilities|FlowControl|RetriggerableDelay 1.0))

(fn Dialogue
  (|CallParentFunction)
  (switch int (Variables|Default|GetDialogueTreeIndex)
    (:0
      (if (Variables|Default|GetAudioCue1Play)
        _
        (else
          (Audio|PlaySound2D "/Game/Audio/VoiceClips/MatthewBryce/Dexter/Happy/Dexter_-_MATTHEW_Happy_7.Dexter_-_MATTHEW_Happy_7" 1.0 1.0 0.0 0 0)
          (Variables|Default|SetAudioCue1Play true)))
      ;[1 0.9823 0] MQ003
      ;;[1 1 1] Dialogue Stage 1
      (bind (_state _optionindex) (CallFunction|AddDialogue "Coordinator Damar" "Well, well, here's the new Scoper come to join us Keppers. Welcome to Colony Atalanta. Arcas Callisto, am I right?" (Utilities|Array|MakeArray "Uh, you have me at a disadvantage, sir. I'm not sure I understand what you mean by 'Scoper'.")))
      (switch Utilities|FlowControl|Switch|SwitchonEnum_DialogueState _state
        (:NewEnumerator0
          (switch int _optionindex
            (:0
              ;;[1 1 1] Dialogue Stage 2
              (bind (_state_2 _optionindex_2) (CallFunction|AddDialogue "Coordinator Damar" "My mistake. My name is Bryce Damar. I coordinate the militia here on Artemis." (Utilities|Array|MakeArray "Continue")))
              (switch Utilities|FlowControl|Switch|SwitchonEnum_DialogueState _state_2
                (:NewEnumerator0
                  (switch int _optionindex_2
                    (:0
                      (if (Variables|Default|GetAudioCue2Play)
                        _
                        (else
                          (Audio|PlaySound2D "/Game/Audio/VoiceClips/MatthewBryce/Dexter/Excited/Dexter_-_MATTHEW_Excited_2.Dexter_-_MATTHEW_Excited_2" 1.0 1.0 0.0 0 0)
                          (Variables|Default|SetAudioCue2Play true)))
                      ;;[1 1 1] Dialogue Stage 3
                      (bind (_state_3 _optionindex_3) (CallFunction|AddDialogue "Coordinator Damar" "Those of us who came on the Key Passage to Artemis, or 'KePA', call ourselves 'Keppers'. You, who came as part of the Secondary Colonisation of the Planet Artemis, or 'SCOPA', are called 'Scopers'." (Utilities|Array|MakeArray "Ah, I see. Kind of like the oldies and the newbies, hey?")))
                      (switch Utilities|FlowControl|Switch|SwitchonEnum_DialogueState _state_3
                        (:NewEnumerator0
                          (switch int _optionindex_3
                            (:0
                              (if (Variables|Default|GetAudioCue3Play)
                                _
                                (else
                                  (Audio|PlaySound2D "/Game/Audio/VoiceClips/MatthewBryce/Dexter/Happy/Dexter_-_MATTHEW_Happy_3.Dexter_-_MATTHEW_Happy_3" 1.0 1.0 0.0 0 0)
                                  (Variables|Default|SetAudioCue3Play true)))
                              ;;[1 1 1] Dialogue Stage 4
                              (bind (_state_4 _optionindex_4) (CallFunction|AddDialogue "Coordinator Damar" "Hah! You're a cheeky bugger. Anyway, I imagine you're trying to make yourself useful around the colony?" (Utilities|Array|MakeArray "Yes, sir")))
                              (switch Utilities|FlowControl|Switch|SwitchonEnum_DialogueState _state_4
                                (:NewEnumerator0
                                  (switch int _optionindex_4
                                    (:0
                                      (if (Variables|Default|GetAudioCue4Play)
                                        _
                                        (else
                                          (Audio|PlaySound2D "/Game/Audio/VoiceClips/MatthewBryce/Tom/Angry/Tom_-_MATTHEW_Angry_1.Tom_-_MATTHEW_Angry_1" 1.0 1.0 0.0 0 0)
                                          (Variables|Default|SetAudioCue4Play true)))
                                      ;;[1 1 1] Dialogue Stage 5
                                      (bind (_state_5 _optionindex_5) (CallFunction|AddDialogue "Coordinator Damar" "Good lad. Part of what we do here is culling the local wildlife that get too close to us. I've seen some animals here that would put a grizzly to shame. One species near us is the Apollon Lykleaver." (Utilities|Array|MakeArray "Even the name sounds scary, sir.")))
                                      (switch Utilities|FlowControl|Switch|SwitchonEnum_DialogueState _state_5
                                        (:NewEnumerator0
                                          (switch int _optionindex_5
                                            (:0
                                              (if (Variables|Default|GetAudioCue5Play)
                                                _
                                                (else
                                                  (Audio|PlaySound2D "/Game/Audio/VoiceClips/MatthewBryce/Dexter/Surprised/Dexter_-_MATTHEW_Surprised_5.Dexter_-_MATTHEW_Surprised_5" 1.0 1.0 0.0 0 0)
                                                  (Variables|Default|SetAudioCue5Play true)))
                                              ;;[1 1 1] Dialogue Stage 6
                                              (bind (_state_6 _optionindex_6) (CallFunction|AddDialogue "Coordinator Damar" "Well, it sure as shit should! Anyway, head back to the hub and access the World Map, and I'll walk you through what we do." (Utilities|Array|MakeArray "Sure thing, sir. I'll contact you once I'm there.")))
                                              (switch Utilities|FlowControl|Switch|SwitchonEnum_DialogueState _state_6
                                                (:NewEnumerator0
                                                  (switch int _optionindex_6
                                                    (:0
                                                      (CallFunction|RemoveDialogueProgress 3)
                                                      (CallFunction|CloseConversation))))))))))))))))))))))))))
    (:1
      (if (Variables|Default|GetAudioCue6Play)
        _
        (else
          (Audio|PlaySound2D "/Game/Audio/VoiceClips/MatthewBryce/Tom/Curious/Tom_-_MATTHEW_Curious_1.Tom_-_MATTHEW_Curious_1" 1.0 1.0 0.0 0 0)
          (Variables|Default|SetAudioCue6Play true)))
      ;[1 0.9823 0] RTS Combat onboarding
      ;;[1 1 1] Dialogue Stage 1
      (bind (_state_7 _optionindex_7) (CallFunction|AddDialogue "Coordinator Damar" "Good afternoon, Scoper. Like we mentioned in the Outpost, the Apollon Lykleavers on Artemis are dangerous, and to keep everyone safe, cullings are required." (Utilities|Array|MakeArray "Absolutely, sir. Can you direct me to any Lykleavers nearby?")))
      (switch Utilities|FlowControl|Switch|SwitchonEnum_DialogueState _state_7
        (:NewEnumerator0
          (switch int _optionindex_7
            (:0
              (bind _asnpc_bryce_damar (Utilities|Casting|CastToNPC_BryceDamar (Components|GetOwner)))
              (Default|PanCamera _asnpc_bryce_damar "-3580.000000,420.000000,1000.000000")
              ;;[1 1 1] Dialogue Stage 2 - SHOW ENEMY
              (bind (_state_8 _optionindex_8) (CallFunction|AddDialogue "Coordinator Damar" "Wouldn't be much of a Militia Coordinator if I didnt, hey? Here's one. Let's take it easy so you can get used to helping coordinate the troops." (Utilities|Array|MakeArray "Continue")))
              (switch Utilities|FlowControl|Switch|SwitchonEnum_DialogueState _state_8
                (:NewEnumerator0
                  (switch int _optionindex_8
                    (:0
                      ;;[1 1 1] Dialogue Stage 3
                      (bind (_state_9 _optionindex_9) (CallFunction|AddDialogue "Coordinator Damar" "Once you have the unit selected, you can direct them to take the bastards out with the right click. Be sure to retreat if you're taking on too much damage." (Utilities|Array|MakeArray "I definitely will, sir, thank you.")))
                      (switch Utilities|FlowControl|Switch|SwitchonEnum_DialogueState _state_9
                        (:NewEnumerator0
                          (switch int _optionindex_9
                            (:0
                              (bind _asnpc_bryce_damar_2 (Utilities|Casting|CastToNPC_BryceDamar (Components|GetOwner)))
                              (Default|PanCamera _asnpc_bryce_damar_2 "-5330.000000,-7170.000000,1000.000000")
                              ;;[1 1 1] Dialogue Stage 3
                              (bind (_state_10 _optionindex_10) (CallFunction|AddDialogue "Coordinator Damar" "If you need more units, click the Main Hub and make your selection. Workers aren't as hardy, so best choose Infantry to fight off enemies." (Utilities|Array|MakeArray "Thanks for the heads up, sir.")))
                              (switch Utilities|FlowControl|Switch|SwitchonEnum_DialogueState _state_10
                                (:NewEnumerator0
                                  (switch int _optionindex_10
                                    (:0
                                      (CallFunction|RemoveDialogueProgress 3)
                                      (CallFunction|CloseConversation)
                                      (bind _foundwidgets (Widget|GetAllWidgetsOfClass "/Game/Blueprints/Dialogue/Widgets/W_Dialogue.W_Dialogue_C" true))
                                      (for _array_element _foundwidgets
                                        (Widget|RemovefromParent _array_element)
                                        (CallFunction|Delay)
                                        (bind _asnpc_bryce_damar_3 (Utilities|Casting|CastToNPC_BryceDamar (Components|GetOwner)))
                                        (Default|EndPan _asnpc_bryce_damar_3)))))))))))))))))))
    (:2
      (if (Variables|Default|GetAudioCue7Play)
        _
        (else
          (Audio|PlaySound2D "/Game/Audio/VoiceClips/MatthewBryce/Dexter/Happy/Dexter_-_MATTHEW_Happy_4.Dexter_-_MATTHEW_Happy_4" 1.0 1.0 0.0 0 0)
          (Variables|Default|SetAudioCue7Play true)))
      ;[1 0.9823 0] Checkin post MQ003
      ;;[1 1 1] Dialogue Stage 5
      (bind (_state_11 _optionindex_11) (CallFunction|AddDialogue "Coordinator Damar" "Good work, lad. Those Lykleavers aren't a massive problem in small numbers, but they can be dangerous in large groups." (Utilities|Array|MakeArray "I can see what you mean, sir. I'll be sure to be careful with them.")))
      (switch Utilities|FlowControl|Switch|SwitchonEnum_DialogueState _state_11
        (:NewEnumerator0
          (switch int _optionindex_11
            (:0
              (if (Variables|Default|GetAudioCue8Play)
                _
                (else
                  (Audio|PlaySound2D "/Game/Audio/VoiceClips/MatthewBryce/Dexter/Excited/Dexter_-_MATTHEW_Excited_5.Dexter_-_MATTHEW_Excited_5" 1.0 1.0 0.0 0 0)
                  (Variables|Default|SetAudioCue8Play true)))
              ;;[1 1 1] Dialogue Stage 6
              (bind (_state_12 _optionindex_12) (CallFunction|AddDialogue "Coordinator Damar" "Smart man. Now, go and check in with Petrine when you're ready. She had to organise a shipment from Colony Atalanta earlier today, so don't waste her time." (Utilities|Array|MakeArray "Understood, sir. The Captain trained me with vids on my way over. I'm used to it.")))
              (switch Utilities|FlowControl|Switch|SwitchonEnum_DialogueState _state_12
                (:NewEnumerator0
                  (switch int _optionindex_12
                    (:0
                      (CallFunction|RemoveDialogueProgress 3)
                      (CallFunction|CloseConversation)
                      (bind _foundwidgets_2 (Widget|GetAllWidgetsOfClass "/Game/Blueprints/Dialogue/Widgets/W_Dialogue.W_Dialogue_C" true))
                      (for _array_element_2 _foundwidgets_2
                        (Widget|RemovefromParent _array_element_2)))))))))))))