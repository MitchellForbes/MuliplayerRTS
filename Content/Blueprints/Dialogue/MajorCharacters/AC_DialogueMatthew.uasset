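; Dialogue component for Commander Vanguarre (Matthew), who gives Arcas the opening Aura Outpost assignment and later the lost equipment retrieval briefing.
; DialogueTreeIndex selects one of two linear, single-option AddDialogue chains, with boolean-guarded voice cues that play once.
; The first tree calls RemoveDialogueProgress before closing.
; The second pans the camera at two stages by casting the owner to NPC_NoahCamenisch, then closes without that call.
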(fn Dialogue
  (|CallParentFunction)
  (Utilities|Casting|CastToBP_ArtemisFrontierGameInstance (Game|GetGameInstance))
  (switch int (Variables|Default|GetDialogueTreeIndex)
    (:0
      ;[1 1 1] This will play the audio ONCE
      (if (Variables|Default|GetAudioCue1Play)
        _
        (else
          (Audio|PlaySound2D "/Game/Audio/VoiceClips/MatthewBryce/Tom/Excited/Tom_-_MATTHEW_Excited_2.Tom_-_MATTHEW_Excited_2" 1.0 1.0 0.0 0 0)
          (Variables|Default|SetAudioCue1Play true)))
      ;[1 0.9922 0] MQ001 Acquisition Dialogue
      ;;[1 1 1] Dialogue Stage 1
      (bind (_state _optionindex) (CallFunction|AddDialogue "Commander Vanguarre" "Howzit, Arcas?" (Utilities|Array|MakeArray "Good morning, sir.")))
      (switch Utilities|FlowControl|Switch|SwitchonEnum_DialogueState _state
        (:NewEnumerator0
          (switch int _optionindex
            (:0
              ;;[1 1 1] Dialogue Stage 2
              (bind (_state_2 _optionindex_2) (CallFunction|AddDialogue "Commander Vanguarre" "Hope you got in off the ASP Odyssey alright. How was the trip?" (Utilities|Array|MakeArray "Warp is still a crazy experience. Shaving a 200 lightyear trip down to 7 months is a big improvement! Lots of prep time for the work here.")))
              (switch Utilities|FlowControl|Switch|SwitchonEnum_DialogueState _state_2
                (:NewEnumerator0
                  (switch int _optionindex_2
                    (:0
                      (if (Variables|Default|GetAudioCue2Play)
                        _
                        (else
                          (Audio|PlaySound2D "/Game/Audio/VoiceClips/MatthewBryce/Dexter/Curious/Dexter_-_MATTHEW_Curious_5.Dexter_-_MATTHEW_Curious_5" 1.0 1.0 0.0 0 0)
                          (Variables|Default|SetAudioCue2Play true)))
                      ;;[1 1 1] Dialogue Stage 3
                      (bind (_state_3 _optionindex_3) (CallFunction|AddDialogue "Commander Vanguarre" "Let's get you to work right away then. I've got a mission for you." (Utilities|Array|MakeArray "What is it, sir?")))
                      (switch Utilities|FlowControl|Switch|SwitchonEnum_DialogueState _state_3
                        (:NewEnumerator0
                          (switch int _optionindex_3
                            (:0
                              ;;[1 1 1] Dialogue Stage 4
                              (bind (_state_4 _optionindex_4) (CallFunction|AddDialogue "Commander Vanguarre" "We've only had Aura Outpost up and running for a couple months now. Certain departments are in need of some help in organising resources. Check in with Captain Acosta to see what she needs." (Utilities|Array|MakeArray "Will do, sir. Where can I find the captain?")))
                              (switch Utilities|FlowControl|Switch|SwitchonEnum_DialogueState _state_4
                                (:NewEnumerator0
                                  (switch int _optionindex_4
                                    (:0
                                      (if (Variables|Default|GetAudioCue3Play)
                                        _
                                        (else
                                          (Audio|PlaySound2D "/Game/Audio/VoiceClips/MatthewBryce/Dexter/Sad/Dexter_-_MATTHEW_Sad_1.Dexter_-_MATTHEW_Sad_1" 1.0 1.0 0.0 0 0)
                                          (Variables|Default|SetAudioCue3Play true)))
                                      ;;[1 1 1] Dialogue Stage 5
                                      (bind (_state_5 _optionindex_5) (CallFunction|AddDialogue "Commander Vanguarre" "At the moment, she's at the Central Plaza. We're currently using it for storage, so excuse the mess." (Utilities|Array|MakeArray "Fantastic, I'll head there now!")))
                                      (switch Utilities|FlowControl|Switch|SwitchonEnum_DialogueState _state_5
                                        (:NewEnumerator0
                                          (switch int _optionindex_5
                                            (:0
                                              (CallFunction|RemoveDialogueProgress 3)
                                              (CallFunction|CloseConversation))))))))))))))))))))))
    (:1
      (if (Variables|Default|GetAudioCue4Play)
        _
        (else
          (Audio|PlaySound2D "/Game/Audio/VoiceClips/MatthewBryce/Dexter/Happy/Dexter_-_MATTHEW_Happy_6.Dexter_-_MATTHEW_Happy_6" 1.0 1.0 0.0 0 0)
          (Variables|Default|SetAudioCue4Play true)))
      ;[1 0.9823 0] Major Item Retrieval Onboarding
      ;;[1 1 1] Dialogue Stage 1
      (bind (_state_6 _optionindex_6) (CallFunction|AddDialogue "Commander Vanguarre" "Excellent work so far, Arcas. Petrine has told me of your work so far. This brings us to our main problem." (Utilities|Array|MakeArray "The captain mentioned losing our equipment on its way over here, sir.")))
      (switch Utilities|FlowControl|Switch|SwitchonEnum_DialogueState _state_6
        (:NewEnumerator0
          (switch int _optionindex_6
            (:0
              ;;[1 1 1] Dialogue Stage 2
              (bind (_state_7 _optionindex_7) (CallFunction|AddDialogue "Commander Vanguarre" "Indeed. A shipment of our final equipment for our infrastructure was jostled by the electic storms Artemis has, and some of the important modules was lost nearby." (Utilities|Array|MakeArray "Where should we look for them, sir?")))
              (switch Utilities|FlowControl|Switch|SwitchonEnum_DialogueState _state_7
                (:NewEnumerator0
                  (switch int _optionindex_7
                    (:0
                      (bind _asnpc_noah_camenisch (Utilities|Casting|CastToNPC_NoahCamenisch (Components|GetOwner)))
                      (Default|PanCamera _asnpc_noah_camenisch "-9880.000000,460.000000,1000.000000")
                      (if (Variables|Default|GetAudioCue5Play)
                        _
                        (else
                          (Audio|PlaySound2D "/Game/Audio/VoiceClips/MatthewBryce/Dexter/Curious/Dexter_-_MATTHEW_Curious_4.Dexter_-_MATTHEW_Curious_4" 1.0 1.0 0.0 0 0)
                          (Variables|Default|SetAudioCue5Play true)))
                      ;;[1 1 1] Dialogue Stage 3
                      (bind (_state_8 _optionindex_8) (CallFunction|AddDialogue "Commander Vanguarre" "To the south is the opening to Rhodos Coast. Intel suggests that the first item is somewhere on the shoreline. After you find that, simply explore the other three areas until you find them all." (Utilities|Array|MakeArray "I won't let you down, sir.")))
                      (switch Utilities|FlowControl|Switch|SwitchonEnum_DialogueState _state_8
                        (:NewEnumerator0
                          (switch int _optionindex_8
                            (:0
                              (bind _asnpc_noah_camenisch_2 (Utilities|Casting|CastToNPC_NoahCamenisch (Components|GetOwner)))
                              (Default|PanCamera _asnpc_noah_camenisch_2 "-5330.000000,-7170.000000,1000.000000")
                              (CallFunction|CloseConversation))))))))))))))))