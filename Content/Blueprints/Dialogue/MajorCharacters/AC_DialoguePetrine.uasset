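; Dialogue component for Captain Petrine Acosta, delivering main quest briefings and hand-overs.
; Completed MQ002 and MQ003 queries on the game instance select one of three dialogue trees.
; Each tree chains nested AddDialogue stages with flag-guarded one-shot voice cues, then removes dialogue progress and closes the conversation.
; The outpost-building tree also blends to overlook and podium cameras and toggles arrows on major building spawners.
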(fn Dialogue
  (|CallParentFunction)
  (bind _outactors (Actor|GetAllActorsOfClass "/Game/QuestSystem/Blueprints/Quest_Base.Quest_Base_C"))
  (for _array_element _outactors
    _)
  (bind _asbp_artemis_frontier_game_instance (Utilities|Casting|CastToBP_ArtemisFrontierGameInstance (Game|GetGameInstance)))
  (if (.ReturnValue (Default|QueryCompletedQuests _asbp_artemis_frontier_game_instance "MQ002"))
    (Variables|Default|SetDialogueTreeIndex 1)
    (if (.ReturnValue (Default|QueryCompletedQuests _asbp_artemis_frontier_game_instance "MQ003"))
      (Variables|Default|SetDialogueTreeIndex 2)))
  (switch int (Variables|Default|GetDialogueTreeIndex)
    (:0
      (if (Variables|Default|GetAudioCue1Play)
        _
        (else
          (Audio|PlaySound2D "/Game/Audio/VoiceClips/Petrine/Holly/Happy/Holly_-_PETRINA_Happy_1.Holly_-_PETRINA_Happy_1" 1.0 1.0 0.0 0 0)
          (Variables|Default|SetAudioCue1Play true)))
      ;[1 0.9647 0] MQ001 Completion Dialogue
      ;
      ; &
      ;
      ; MQ002 Acquisition Dialogue
      ;;[1 1 1] Dialogue Stage 1
      (bind (_state _optionindex) (CallFunction|AddDialogue "Captain Acosta" "Hello, Arcas. Good to see you again!" (Utilities|Array|MakeArray "You too, Captain. I heard you could use some help?")))
      (switch Utilities|FlowControl|Switch|SwitchonEnum_DialogueState _state
        (:NewEnumerator0
          (switch int _optionindex
            (:0
              (if (Variables|Default|GetAudioCue2Play)
                _
                (else
                  (Audio|PlaySound2D "/Game/Audio/VoiceClips/Petrine/Holly/Curious/Holly_-_PETRINA_Curious_4.Holly_-_PETRINA_Curious_4" 1.0 1.0 0.0 0 0)
                  (Variables|Default|SetAudioCue2Play true)))
              ;;[1 1 1] Dialogue Stage 2
              (bind (_state_2 _optionindex_2) (CallFunction|AddDialogue "Captain Acosta" "Indeed. We're slated to receive more colonists in the next few months, so we need to make sure we have enough industry up and running here in the outpost." (Utilities|Array|MakeArray "Of course. What do we need?")))
              (switch Utilities|FlowControl|Switch|SwitchonEnum_DialogueState _state_2
                (:NewEnumerator0
                  (switch int _optionindex_2
                    (:0
                      (if (Variables|Default|GetAudioCue3Play)
                        _
                        (else
                          (Audio|PlaySound2D "/Game/Audio/VoiceClips/Petrine/Holly/Happy/Holly_-_PETRINA_Happy_5.Holly_-_PETRINA_Happy_5" 1.0 1.0 0.0 0 0)
                          (Variables|Default|SetAudioCue3Play true)))
                      ;;[1 1 1] Dialogue Stage 3
                      (bind (_state_3 _optionindex_3) (CallFunction|AddDialogue "Captain Acosta" "I want you to assist with mining 500 of the local minerals. We set Colony Atalanta up near to some to the WEST, so we can get started quickly." (Utilities|Array|MakeArray "Absolutely. Where do I go to begin?")))
                      (switch Utilities|FlowControl|Switch|SwitchonEnum_DialogueState _state_3
                        (:NewEnumerator0
                          (switch int _optionindex_3
                            (:0
                              (if (Variables|Default|GetAudioCue4Play)
                                _
                                (else
                                  (Audio|PlaySound2D "/Game/Audio/VoiceClips/Petrine/Holly/Excited/Holly_-_PETRINA_Excited_6.Holly_-_PETRINA_Excited_6" 1.0 1.0 0.0 0 0)
                                  (Variables|Default|SetAudioCue4Play true)))
                              ;;[1 1 1] Dialogue Stage 4
                              (bind (_state_4 _optionindex_4) (CallFunction|AddDialogue "Captain Acosta" "Head back into the Main Hub, there's a console where you can communicate with the mining corps. 
Now on with it, the madness never stops with Earth 2.0!" (Utilities|Array|MakeArray "Heh, I'm beginning to get that impression...")))
                              (switch Utilities|FlowControl|Switch|SwitchonEnum_DialogueState _state_4
                                (:NewEnumerator0
                                  (switch int _optionindex_4
                                    (:0
                                      (if (Variables|Default|GetAudioCue5Play)
                                        _
                                        (else
                                          (Audio|PlaySound2D "/Game/Audio/VoiceClips/Petrine/Holly/Nervous/Holly_-_PETRINA_Nervous_1.Holly_-_PETRINA_Nervous_1" 1.0 1.0 0.0 0 0)
                                          (Variables|Default|SetAudioCue5Play true)))
                                      ;;[1 1 1] Dialogue Stage 5
                                      (bind _state_5 (CallFunction|AddDialogue "Captain Acosta" "Matthew does my head in sometimes, I swear... Also, Scout Lieutenant Camenisch will give you the run down of how extraction works. He's... eccentric, but highly effective." (Utilities|Array|MakeArray "Understood, ma'am.")))
                                      (switch Utilities|FlowControl|Switch|SwitchonEnum_DialogueState _state_5
                                        (:NewEnumerator0
                                          (CallFunction|RemoveDialogueProgress 4)
                                          (CallFunction|CloseConversation)
                                          (Input|SetInputModeGameOnly 0 false))))))))))))))))))))
    (:1
      (if (Variables|Default|GetAudioCue6Play)
        _
        (else
          (Audio|PlaySound2D "/Game/Audio/VoiceClips/Petrine/Holly/Happy/Holly_-_PETRINA_Happy_8.Holly_-_PETRINA_Happy_8" 1.0 1.0 0.0 0 0)
          (Variables|Default|SetAudioCue6Play true)))
      ;[1 0.9647 0] MQ002-MQ003 HandOver Dialogue
      ;;[1 1 1] Dialogue Stage 1
      (bind (_state_6 _optionindex_5) (CallFunction|AddDialogue "Captain Acosta" "Thanks for that, Arcas. Over time, we'll add to the colony as we get more colonists, and who knows? Maybe we'll start making little Artemisians soon!" (Utilities|Array|MakeArray "Hah! Maybe one day soon, indeed. My yia-yia has already demanded I give her grandkids.")))
      (switch Utilities|FlowControl|Switch|SwitchonEnum_DialogueState _state_6
        (:NewEnumerator0
          (switch int _optionindex_5
            (:0
              ;;[1 1 1] Dialogue Stage 2
              (bind (_state_7 _optionindex_6) (CallFunction|AddDialogue "Captain Acosta" "Reminds me of my family too. 
 
In the meantime, head over to our militia coordinator, Bryce Damar. You'll find him over at the Helipad next to the Main Hub." (Utilities|Array|MakeArray "What is it that he needs?")))
              (switch Utilities|FlowControl|Switch|SwitchonEnum_DialogueState _state_7
                (:NewEnumerator0
                  (switch int _optionindex_6
                    (:0
                      (if (Variables|Default|GetAudioCue7Play)
                        _
                        (else
                          (Audio|PlaySound2D "/Game/Audio/VoiceClips/Petrine/Holly/Sad/Holly_-_PETRINA_Sad_4.Holly_-_PETRINA_Sad_4" 1.0 1.0 0.0 0 0)
                          (Variables|Default|SetAudioCue7Play true)))
                      ;;[1 1 1] Dialogue Stage 2
                      (bind (_state_8 _optionindex_7) (CallFunction|AddDialogue "Captain Acosta" "He's been moaning about some of the wildlife pressing on the colony recently. He could always do with some assistance organising their culling." (Utilities|Array|MakeArray "Of course, I'll be sure to check in with him.")))
                      (switch Utilities|FlowControl|Switch|SwitchonEnum_DialogueState _state_8
                        (:NewEnumerator0
                          (switch int _optionindex_7
                            (:0
                              (CallFunction|RemoveDialogueProgress 3)
                              (CallFunction|CloseConversation))))))))))))))
    (:2
      (if (Variables|Default|GetAudioCue8Play)
        _
        (else
          (Audio|PlaySound2D "/Game/Audio/VoiceClips/Petrine/Holly/Angry/Holly_-_PETRINA_Angry_2.Holly_-_PETRINA_Angry_2" 1.0 1.0 0.0 0 0)
          (Variables|Default|SetAudioCue8Play true)))
      ;[1 0.9647 0] Explanation of MQ004
      ;;[1 1 1] Dialogue Stage 1
      (bind (_state_9 _optionindex_8) (CallFunction|AddDialogue "Captain Acosta" "Yes, what is it, Arcas?" (Utilities|Array|MakeArray "Sorry to disturb you, ma'am. I've checked in with Coordinator Damar, and he let me know that I'm ready for the next step. ")))
      (switch Utilities|FlowControl|Switch|SwitchonEnum_DialogueState _state_9
        (:NewEnumerator0
          (switch int _optionindex_8
            (:0
              ;;[1 1 1] Dialogue Stage 2
              (bind (_state_10 _optionindex_9) (CallFunction|AddDialogue "Captain Acosta" "Ah, yes. Part of what we do here on Artemis is setting up Outposts. We can get shipments from Earth and Colony Atalanta, but ultimately, we need to be self sufficient." (Utilities|Array|MakeArray "That makes sense. Are there any particular priorities?")))
              (switch Utilities|FlowControl|Switch|SwitchonEnum_DialogueState _state_10
                (:NewEnumerator0
                  (switch int _optionindex_9
                    (:0
                      (if (Variables|Default|GetAudioCue9Play)
                        _
                        (else
                          (Audio|PlaySound2D "/Game/Audio/VoiceClips/Petrine/Holly/Excited/Holly_-_PETRINA_Excited_2.Holly_-_PETRINA_Excited_2" 1.0 1.0 0.0 0 0)
                          (Variables|Default|SetAudioCue9Play true)))
                      ;;[1 1 1] Dialogue Stage 3 - CAMERA MOVES TO SHOW PLOTS ABOVE
                      (bind (_state_11 _optionindex_10) (CallFunction|AddDialogue "Captain Acosta" "There are. We have four plots set up in the outpost:  " (Utilities|Array|MakeArray "Continue")))
                      (switch Utilities|FlowControl|Switch|SwitchonEnum_DialogueState _state_11
                        (:NewEnumerator0
                          (switch int _optionindex_10
                            (:0
                              (bind _asnpc_petrine_acosta (Utilities|Casting|CastToNPC_PetrineAcosta (Components|GetOwner)))
                              (Game|Player|SetViewTargetwithBlend (Game|GetPlayerController 0) (Variables|/Game/Characters/NPCs/MajorCharacters/NPC_PetrineAcosta.NPC_PetrineAcosta_C|GetOverlookCamera _asnpc_petrine_acosta) 1.5 "VTBlend_Linear" 0.0 true)
                              (bind _outactors_2 (Actor|GetAllActorsOfClass "/Game/Blueprints/Buildings/ThirdPersonBuildings/MajorBuildings/BP_BuildingSpawnerMajor.BP_BuildingSpawnerMajor_C"))
                              (for _array_element_2 _outactors_2
                                (Default|ActivateArrows _array_element_2)
                                ;;[1 1 1] Dialogue Stage 4
                                (bind (_state_12 _optionindex_11) (CallFunction|AddDialogue "Captain Acosta" "Alloy Fabrication;" (Utilities|Array|MakeArray "Continue")))
                                (switch Utilities|FlowControl|Switch|SwitchonEnum_DialogueState _state_12
                                  (:NewEnumerator0
                                    (switch int _optionindex_11
                                      (:0
                                        ;;[1 1 1] Dialogue Stage 5
                                        (bind (_state_13 _optionindex_12) (CallFunction|AddDialogue "Captain Acosta" "Food Processing; " (Utilities|Array|MakeArray "Continue")))
                                        (switch Utilities|FlowControl|Switch|SwitchonEnum_DialogueState _state_13
                                          (:NewEnumerator0
                                            (switch int _optionindex_12
                                              (:0
                                                ;;[1 1 1] Dialogue Stage 6
                                                (bind (_state_14 _optionindex_13) (CallFunction|AddDialogue "Captain Acosta" "Mineral Extraction;" (Utilities|Array|MakeArray "Continue")))
                                                (switch Utilities|FlowControl|Switch|SwitchonEnum_DialogueState _state_14
                                                  (:NewEnumerator0
                                                    (switch int _optionindex_13
                                                      (:0
                                                        ;;[1 1 1] Dialogue Stage 7
                                                        (bind (_state_15 _optionindex_14) (CallFunction|AddDialogue "Captain Acosta" "and Oil Refining." (Utilities|Array|MakeArray "Continue")))
                                                        (switch Utilities|FlowControl|Switch|SwitchonEnum_DialogueState _state_15
                                                          (:NewEnumerator0
                                                            (switch int _optionindex_14
                                                              (:0
                                                                (bind _asbp_third_person_character (Utilities|Casting|CastToBP_ThirdPersonCharacter (Game|GetPlayerCharacter 0)))
                                                                (Game|Player|SetViewTargetwithBlend (Game|GetPlayerController 0) _asbp_third_person_character 1.5 "VTBlend_Linear" 0.0 true)
                                                                (bind _outactors_3 (Actor|GetAllActorsOfClass "/Game/Blueprints/Buildings/ThirdPersonBuildings/MajorBuildings/BP_BuildingSpawnerMajor.BP_BuildingSpawnerMajor_C"))
                                                                (for _array_element_3 _outactors_3
                                                                  (Default|DeactivateArrows _array_element_3)
                                                                  (if (Variables|Default|GetAudioCue10Play)
                                                                    _
                                                                    (else
                                                                      (Audio|PlaySound2D "/Game/Audio/VoiceClips/Petrine/Holly/Nervous/Holly_-_PETRINA_Nervous_1.Holly_-_PETRINA_Nervous_1" 1.0 1.0 0.0 0 0)
                                                                      (Variables|Default|SetAudioCue10Play true)))
                                                                  ;;[1 1 1] Dialogue Stage 7
                                                                  (bind (_state_16 _optionindex_15) (CallFunction|AddDialogue "Captain Acosta" "The deal is that each of these buildings needs a specific material found on Artemis... and we lost them on their way here." (Utilities|Array|MakeArray "*Hah! Of course they were.* Sorry to hear that, ma'am.")))
                                                                  (switch Utilities|FlowControl|Switch|SwitchonEnum_DialogueState _state_16
                                                                    (:NewEnumerator0
                                                                      (switch int _optionindex_15
                                                                        (:0
                                                                          (if (Variables|Default|GetAudioCue11Play)
                                                                            _
                                                                            (else
                                                                              (Audio|PlaySound2D "/Game/Audio/VoiceClips/Petrine/Holly/Curious/Holly_-_PETRINA_Curious_6.Holly_-_PETRINA_Curious_6" 1.0 1.0 0.0 0 0)
                                                                              (Variables|Default|SetAudioCue11Play true)))
                                                                          ;;[1 1 1] Dialogue Stage 7
                                                                          (bind (_state_17 _optionindex_16) (CallFunction|AddDialogue "Captain Acosta" "Let's get onto it then. Outpost Aura is in New Thessaly. To our south is Rhodos Coast, to the north is Kione's Rift, and to our east is the Haphaestus Fissure and New Foloi Forest." (Utilities|Array|MakeArray "And I imagine that the equipment has fallen in each of these locations?")))
                                                                          (switch Utilities|FlowControl|Switch|SwitchonEnum_DialogueState _state_17
                                                                            (:NewEnumerator0
                                                                              (switch int _optionindex_16
                                                                                (:0
                                                                                  ;;[1 1 1] Dialogue Stage 7
                                                                                  (bind (_state_18 _optionindex_17) (CallFunction|AddDialogue "Captain Acosta" "Correct. Liaise with the corps on the World Map, and Matthew will talk you through the process." (Utilities|Array|MakeArray "Will do. After I get them, how will we build the structures?")))
                                                                                  (switch Utilities|FlowControl|Switch|SwitchonEnum_DialogueState _state_18
                                                                                    (:NewEnumerator0
                                                                                      (switch int _optionindex_17
                                                                                        (:0
                                                                                          (bind _asnpc_petrine_acosta_2 (Utilities|Casting|CastToNPC_PetrineAcosta (Components|GetOwner)))
                                                                                          (Game|Player|SetViewTargetwithBlend (Game|GetPlayerController 0) (Variables|/Game/Characters/NPCs/MajorCharacters/NPC_PetrineAcosta.NPC_PetrineAcosta_C|GetPodiumCamera _asnpc_petrine_acosta_2) 1.5 "VTBlend_Linear" 0.0 true)
                                                                                          (if (Variables|Default|GetAudioCue12Play)
                                                                                            _
                                                                                            (else
                                                                                              (Audio|PlaySound2D "/Game/Audio/VoiceClips/Petrine/Holly/Excited/Holly_-_PETRINA_Excited_7.Holly_-_PETRINA_Excited_7" 1.0 1.0 0.0 0 0)
                                                                                              (Variables|Default|SetAudioCue12Play true)))
                                                                                          ;;[1 1 1] Dialogue Stage 7
                                                                                          (bind (_state_19 _optionindex_18) (CallFunction|AddDialogue "Captain Acosta" "Head to this podium. When you do, you can select which building to have built and the required resources to do so." (Utilities|Array|MakeArray "Understood. Thanks for the explanation, ma'am.")))
                                                                                          (switch Utilities|FlowControl|Switch|SwitchonEnum_DialogueState _state_19
                                                                                            (:NewEnumerator0
                                                                                              (switch int _optionindex_18
                                                                                                (:0
                                                                                                  (CallFunction|RemoveDialogueProgress 3)
                                                                                                  (CallFunction|CloseConversation)
                                                                                                  (Input|SetInputModeGameOnly 0 false))))))))))))))))))))))))))))))))))))))))))))))))))