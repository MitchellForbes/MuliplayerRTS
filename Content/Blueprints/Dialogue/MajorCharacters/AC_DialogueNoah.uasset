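; Dialogue component for Scout Lieutenant Noah Camenisch, who delivers the RTS map onboarding and a follow-up once 250 minerals are gathered.
; DialogueTreeIndex selects the tree, and each AddDialogue stage nests under the previous reply, with flag-guarded one-shot voice cues.
; The tutorial pans the camera through the owning NPC to show resources and building, then ends the pan.
; Both trees close the conversation and remove dialogue widgets.
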(fn Dialogue
  (|CallParentFunction)
  (switch int (Variables|Default|GetDialogueTreeIndex)
    (:0
      (if (Variables|Default|GetAudioCue1Play)
        _
        (else
          (Audio|PlaySound2D "/Game/Audio/VoiceClips/Noah/Dexter/Excited/Dexter_-_NOAH_Excited_3.Dexter_-_NOAH_Excited_3" 1.0 1.0 0.0 0 0)
          (Variables|Default|SetAudioCue1Play true)))
      ;[1 0.9823 0] RTS Map onboarding
      ;;[1 1 1] Dialogue Stage 1
      (bind (_state _optionindex) (CallFunction|AddDialogue "???" "Grüezi, new scout! I mean to say, 'hi'. My name is Noah, SCOUT EXTRAORDINAIRE!" (Utilities|Array|MakeArray "Hi there, uh, 'Scout Extraordinaire'. You are Scout Lieutenant Camenisch, yes?")))
      (switch Utilities|FlowControl|Switch|SwitchonEnum_DialogueState _state
        (:NewEnumerator0
          (switch int _optionindex
            (:0
              (if (Variables|Default|GetAudioCue2Play)
                _
                (else
                  (Audio|PlaySound2D "/Game/Audio/VoiceClips/Noah/Dexter/Surprised/Dexter_-_NOAH_Surprised_1.Dexter_-_NOAH_Surprised_1" 1.0 1.0 0.0 0 0)
                  (Variables|Default|SetAudioCue2Play true)))
              ;;[1 1 1] Dialogue Stage 2
              (bind (_state_2 _optionindex_2) (CallFunction|AddDialogue "Scout Lieutenant Camenisch" "Most certainly! I see you're helping out administer what the colony needs, so I'm here to point out a few... pointers, that will help you understand what we do here." (Utilities|Array|MakeArray "Thanks, Noah!")))
              (switch Utilities|FlowControl|Switch|SwitchonEnum_DialogueState _state_2
                (:NewEnumerator0
                  (switch int _optionindex_2
                    (:0
                      (if (Variables|Default|GetAudioCue3Play)
                        _
                        (else
                          (Audio|PlaySound2D "/Game/Audio/VoiceClips/Noah/Dexter/Happy/Dexter_-_NOAH_Happy_7.Dexter_-_NOAH_Happy_7" 1.0 1.0 0.0 0 0)
                          (Variables|Default|SetAudioCue3Play true)))
                      ;;[1 1 1] Dialogue Stage 3 - SHOW UNITS
                      (bind (_state_3 _optionindex_3) (CallFunction|AddDialogue "Scout Lieutenant Camenisch" "First of all, you can direct our intrepid explorers individually, or as a group by clicking and dragging over them. Right click on any resources for them to go to and extract." (Utilities|Array|MakeArray "Continue")))
                      (switch Utilities|FlowControl|Switch|SwitchonEnum_DialogueState _state_3
                        (:NewEnumerator0
                          (switch int _optionindex_3
                            (:0
                              ;;[1 1 1] Dialogue Stage 4
                              (bind (_state_4 _optionindex_4) (CallFunction|AddDialogue "Scout Lieutenant Camenisch" "What's this you say? You are after 250 minerals? That is, how we say in Switzerland, the Hammer!" (Utilities|Array|MakeArray "Hah, sure. Captain Acosta said they were to the West of the colony.")))
                              (switch Utilities|FlowControl|Switch|SwitchonEnum_DialogueState _state_4
                                (:NewEnumerator0
                                  (switch int _optionindex_4
                                    (:0
                                      (bind _asnpc_noah_camenisch (Utilities|Casting|CastToNPC_NoahCamenisch (Components|GetOwner)))
                                      (Default|PanCamera _asnpc_noah_camenisch "-3760.000000,-13080.000000,1000.000000")
                                      ;;[1 1 1] Dialogue Stage 5 - SHOW MINERAL DEPOSIT
                                      (bind (_state_5 _optionindex_5) (CallFunction|AddDialogue "Scout Lieutenant Camenisch" "Indeed, we do have some, near Mt. Othrys. It is a simple trip over there. New Thessaly is one of the safer areas on Artemis." (Utilities|Array|MakeArray "Understood. Anything else?")))
                                      (switch Utilities|FlowControl|Switch|SwitchonEnum_DialogueState _state_5
                                        (:NewEnumerator0
                                          (switch int _optionindex_5
                                            (:0
                                              (bind _asnpc_noah_camenisch_2 (Utilities|Casting|CastToNPC_NoahCamenisch (Components|GetOwner)))
                                              (Default|PanCamera _asnpc_noah_camenisch_2 "228.000000,-13745.000000,1000.000000")
                                              ;;[1 1 1] Dialogue Stage 5 - SHOW ALLOY DEPOSIT
                                              (bind (_state_6 _optionindex_6) (CallFunction|AddDialogue "Scout Lieutenant Camenisch" "Alos, behold Artemite! We use this for our mechsuits, so you'll need this to get more units!" (Utilities|Array|MakeArray "Interesting...")))
                                              (switch Utilities|FlowControl|Switch|SwitchonEnum_DialogueState _state_6
                                                (:NewEnumerator0
                                                  (switch int _optionindex_6
                                                    (:0
                                                      (bind _asnpc_noah_camenisch_3 (Utilities|Casting|CastToNPC_NoahCamenisch (Components|GetOwner)))
                                                      (Default|PanCamera _asnpc_noah_camenisch_3 "1094.000000,-12344.000000,1000.000000")
                                                      ;;[1 1 1] Dialogue Stage 5 - SHOW Food DEPOSIT
                                                      (bind (_state_7 _optionindex_7) (CallFunction|AddDialogue "Scout Lieutenant Camenisch" "It very much is! Lastly, savour the image of the bountiful food of this world! Greatly nutritious, you could last alone for days!" (Utilities|Array|MakeArray "Of course one could... How would I get more units?")))
                                                      (switch Utilities|FlowControl|Switch|SwitchonEnum_DialogueState _state_7
                                                        (:NewEnumerator0
                                                          (switch int _optionindex_7
                                                            (:0
                                                              (bind _asnpc_noah_camenisch_4 (Utilities|Casting|CastToNPC_NoahCamenisch (Components|GetOwner)))
                                                              (Default|PanCamera _asnpc_noah_camenisch_4 "-5330.000000,-7170.000000,1000.000000")
                                                              (if (Variables|Default|GetAudioCue4Play)
                                                                _
                                                                (else
                                                                  (Audio|PlaySound2D "/Game/Audio/VoiceClips/Noah/Dexter/Excited/Dexter_-_NOAH_Excited_5.Dexter_-_NOAH_Excited_5" 1.0 1.0 0.0 0 0)
                                                                  (Variables|Default|SetAudioCue4Play true)))
                                                              ;;[1 1 1] Dialogue Stage 6
                                                              (bind (_state_8 _optionindex_8) (CallFunction|AddDialogue "Scout Lieutenant Camenisch" "If you click on the Outpost, you will see a selection of buildings appear, and you can apply them where you like." (Utilities|Array|MakeArray "Ah, so this can extend where I can deliver resources?")))
                                                              (switch Utilities|FlowControl|Switch|SwitchonEnum_DialogueState _state_8
                                                                (:NewEnumerator0
                                                                  (switch int _optionindex_8
                                                                    (:0
                                                                      ;;[1 1 1] Dialogue Stage 7
                                                                      (bind (_state_9 _optionindex_9) (CallFunction|AddDialogue "Scout Lieutenant Camenisch" "Ja! Keep in mind that you will need food and alloy resources to build these. Cannot have the men going hungry when they work, ja?!" (Utilities|Array|MakeArray "Uh... ja. Thank you, Noah, I'll keep that in mind.")))
                                                                      (switch Utilities|FlowControl|Switch|SwitchonEnum_DialogueState _state_9
                                                                        (:NewEnumerator0
                                                                          (switch int _optionindex_9
                                                                            (:0
                                                                              (if (Variables|Default|GetAudioCue5Play)
                                                                                _
                                                                                (else
                                                                                  (Audio|PlaySound2D "/Game/Audio/VoiceClips/Noah/Tom/Excited/Tom_-_NOAH_Excited_1.Tom_-_NOAH_Excited_1" 1.0 1.0 0.0 0 0)
                                                                                  (Variables|Default|SetAudioCue5Play true)))
                                                                              ;;[1 1 1] Dialogue Stage 8
                                                                              (bind (_state_10 _optionindex_10) (CallFunction|AddDialogue "Scout Lieutenant Camenisch" "You are so very welcome, new colonist!" (Utilities|Array|MakeArray "See you around, Noah.")))
                                                                              (switch Utilities|FlowControl|Switch|SwitchonEnum_DialogueState _state_10
                                                                                (:NewEnumerator0
                                                                                  (switch int _optionindex_10
                                                                                    (:0
                                                                                      (bind _asnpc_noah_camenisch_5 (Utilities|Casting|CastToNPC_NoahCamenisch (Components|GetOwner)))
                                                                                      (Default|EndPan _asnpc_noah_camenisch_5)
                                                                                      (CallFunction|RemoveDialogueProgress 10)
                                                                                      (CallFunction|CloseConversation)
                                                                                      (bind _foundwidgets (Widget|GetAllWidgetsOfClass "/Game/Blueprints/Dialogue/Widgets/W_Dialogue.W_Dialogue_C" true))
                                                                                      (for _array_element _foundwidgets
                                                                                        (Widget|RemovefromParent _array_element)))))))))))))))))))))))))))))))))))))))))))
    (:1
      (if (Variables|Default|GetAudioCue6Play)
        _
        (else
          (Audio|PlaySound2D "/Game/Audio/VoiceClips/Noah/Dexter/Happy/Dexter_-_NOAH_Happy_7.Dexter_-_NOAH_Happy_7" 1.0 1.0 0.0 0 0)
          (Variables|Default|SetAudioCue6Play true)))
      ;[1 0.9823 0] RTS Map onboarding
      ;;[1 1 1] Dialogue Stage 1
      (bind (_state_11 _optionindex_11) (CallFunction|AddDialogue "Scout Lieutenant Camenisch" "Congratulations, young lad! Now that you have 250 minerals, you can now go back to Captain Acosta and see what she needs them for." (Utilities|Array|MakeArray "Of course. Thanks, Noah!")))
      (switch Utilities|FlowControl|Switch|SwitchonEnum_DialogueState _state_11
        (:NewEnumerator0
          (switch int _optionindex_11
            (:0
              (CallFunction|CloseConversation)
              (bind _foundwidgets_2 (Widget|GetAllWidgetsOfClass "/Game/Blueprints/Dialogue/Widgets/W_Dialogue.W_Dialogue_C" true))
              (for _array_element_2 _foundwidgets_2
                (Widget|RemovefromParent _array_element_2)))))))))