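; UnitBuildingBase is a base building unit that opens a base menu when left-clicked in an RTS.
; On click it clears the player controller's unit selection, runs the parent click logic, moves the camera to the building and disables zoom.
; It creates a BaseMenuUI widget for the viewport, then removes and clears it when the parent-extended IsSelected event reports deselection.
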(event EventIsSelected
  (params (IsSelected :type Boolean))
  (|CallParentFunction IsSelected)
  (if (not IsSelected)
    (Widget|RemovefromParent (Variables|Default|GetBaseMenu))
    (Variables|Default|SetBaseMenu 0)))

(event MouseInput|EventActorOnClicked
  (params (ButtonPressed :type Key%20Structure :default "None"))
  (if (== ButtonPressed "LeftMouseButton")
    (bind _aspc_rts (Utilities|Casting|CastToPC_RTS (Game|GetPlayerController 0)))
    (Default|ClearUnitSelection _aspc_rts)
    (|CallParentFunction ButtonPressed)
    (Default|SetCameraLocation (Variables|Default|GetAs%20PC%20RTS) (Transformation|GetActorLocation))
    (bind _returnvalue (UserInterface|CreateWidget "/Game/UI/BaseBuildingUI/BaseMenuUI.BaseMenuUI_C"))
    (bind _output_get (Variables|Default|SetBaseMenu _returnvalue))
    (UserInterface|Viewport|AddtoViewport _output_get 0)
    (Variables|/Game/Blueprints/Player/PC_RTS.PC_RTS_C|SetIsZoomEnabled (Variables|Default|GetAs%20PC%20RTS) false)))

(fn ConstructionScript
  (|CallParentFunction))