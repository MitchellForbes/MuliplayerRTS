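; Infantry unit that works as a resource gatherer, shuttling between a resource node and its team's buildings.
; SetisWorking picks the node and searches for the closest same-team building as dropoff.
; Collect runs a timer before carrying the resource back; Dropoff credits the team's player controller and returns the unit to the node.
; Multicast events sync particles, audio and the carried-resource material; SetNotWorking cancels collection.
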(event Custom|ResourceCollected
  (Utilities|Time|ClearandInvalidateTimerbyHandle (Variables|Default|GetResourceCollectTimer))
  (Variables|Default|SetHasResource? true)
  (CallFunction|UnitMove (Transformation|GetActorLocation (Variables|Default|GetDropOffBuilding)))
  (CallFunction|MulticastStopCollecting))

(event Custom|MulticastStartCollecting
  ;[1 1 1] multicast start collecting
  (Components|Activation|SetActive (Variables|Default|GetParticleSystem) true false)
  (Audio|Components|Audio|Play (Variables|Default|GetAudio) 0.0))

(event Custom|MulticastStopCollecting
  ;[1 1 1] multicast done collecting
  (Components|Activation|SetActive (Variables|Default|GetParticleSystem) false false)
  (Audio|Components|Audio|Stop (Variables|Default|GetAudio))
  (Rendering|Material|SetMaterial (Variables|Default|GetResource) 0 "/Game/StarterContent/Materials/M_Metal_Gold.M_Metal_Gold"))

(event Custom|MulticastDropOff
  ;[1 1 1] multicast dropoff
  (Rendering|Material|SetMaterial (Variables|Default|GetResource) 0 "/Game/StarterContent/Materials/M_Basic_Wall.M_Basic_Wall"))

(event Custom|MulticastUnitNotWorking
  ;[1 1 1] Multicast unit not working
  (Components|Activation|SetActive (Variables|Default|GetParticleSystem) false false)
  (Audio|Components|Audio|Stop (Variables|Default|GetAudio)))

(event EventSetisWorking
  (params (ResourceNode :type Actor%20Object%20Reference))
  (Variables|Default|SetIsWorking? true)
  (Variables|Default|SetResourceNode ResourceNode)
  ;[1 1 1] Change for dropoff point
  (bind _outactors (Actor|GetAllActorsOfClass "/Game/Blueprints/Buildings/RTSBuilding/BP_Parent_Building.BP_Parent_Building_C"))
  (for _array_element _outactors
    ;[1 1 1] Find Closest dropoff building
    (bind _teamnumber (Default|GetTeam _array_element))
    (if (== _teamnumber (Variables|Default|GetTeamNumber))
      (if (< (Transformation|GetDistanceTo _array_element self) (Variables|Default|GetClosestDropOff))
        (Variables|Default|SetDropOffBuilding _array_element)
        (Variables|Default|SetClosestDropOff (Transformation|GetDistanceTo _array_element self)))))
  (if (Variables|Default|GetHasResource?)
    ;[1 1 1] Move to dropoff
    (CallFunction|UnitMove (Transformation|GetActorLocation (Variables|Default|GetDropOffBuilding)))
    (else
      ;[1 1 1] move to resource
      (CallFunction|UnitMove (Transformation|GetActorLocation (Variables|Default|GetResourceNode))))))

(event EventSetNotWorking
  (Variables|Default|SetIsWorking? false)
  (Utilities|Time|ClearandInvalidateTimerbyHandle (Variables|Default|GetResourceCollectTimer))
  (CallFunction|MulticastUnitNotWorking))

(event EventCollect
  (if (Variables|Default|GetIsWorking?)
    (if (Variables|Default|GetHasResource?)
      ;[1 1 1] has resource, move to dropoff
      (CallFunction|UnitMove (Transformation|GetActorLocation (Variables|Default|GetDropOffBuilding)))
      (elif (not (Utilities|Time|IsValidTimerHandle (Variables|Default|GetResourceCollectTimer)))
        ;[1 1 1] stop movement
        (CallFunction|UnitMove (Transformation|GetActorLocation))
        (CallFunction|MulticastStartCollecting)
        (bind _returnvalue (Utilities|Time|SetTimerbyEvent (delegate Custom|ResourceCollected) 4.0))
        (Variables|Default|SetResourceCollectTimer _returnvalue)))))

(event EventDropoff
  (if (Variables|Default|GetIsWorking?)
    (if (Variables|Default|GetHasResource?)
      (Class|BPIInterface|IncrementResourceAmount(Message) (Game|GetPlayerController (Variables|Default|GetTeamNumber)) 10 (Variables|Default|GetResourceName))
      (Variables|Default|SetHasResource? false)
      (CallFunction|MulticastDropOff)
      (CallFunction|UnitMove (Transformation|GetActorLocation (Variables|Default|GetResourceNode)))
      (else
        ;[1 1 1] Move to resource, if no resource
        (CallFunction|UnitMove (Transformation|GetActorLocation (Variables|Default|GetResourceNode)))))))

(fn ConstructionScript
  (|CallParentFunction)
  (Utilities|Array|Add (Variables|Default|GetMeshForColouring) (Variables|Default|GetBody)))

(fn IsonMyTeam?
  (params (TeamNumber :type Integer))
  (return false))