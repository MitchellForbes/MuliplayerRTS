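; Base class for player RTS units, handling selection, movement, combat and health.
; Clicks update selection through PC_RTS, and the selection decal shows the state.
; AI MoveTo drives moves and attacks, with failed moves falling back to the nearest free formation position from PC_RTS.
; AttackBox overlap with the target starts timed damage on BP_EnemyParentClass with alternating animations, while a camera-oriented health bar shows damage until death destroys the unit.
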(event OnComponentEndOverlap(AttackBox)
  (params (OverlappedComponent :type Primitive%20Component%20Object%20Reference) (OtherActor :type Actor%20Object%20Reference) (OtherComp :type Primitive%20Component%20Object%20Reference) (OtherBodyIndex :type Integer))
  (if (== OtherActor (Variables|UnitCombat|GetUnitInRange))
    (Utilities|Time|SetTimerbyFunctionName 0 "DamageUnit" 1.0)
    (Variables|UnitCombat|SetUnitInRange 0)))

(event OnComponentBeginOverlap(AttackBox)
  (params (OverlappedComponent :type Primitive%20Component%20Object%20Reference) (OtherActor :type Actor%20Object%20Reference) (OtherComp :type Primitive%20Component%20Object%20Reference) (OtherBodyIndex :type Integer) (bFromSweep :type Boolean) (SweepResult :type Hit%20Result%20Structure%20%28by%20ref%29))
  (if (== OtherActor (Variables|UnitCombat|GetUnitInRange))
    (CallFunction|Attack)))

(event Custom|Attack
  (if (!= self (Variables|UnitCombat|GetUnitInRange))
    ;[1 1 1] Attack Delay
    (Utilities|Time|SetTimerbyFunctionName 0 "DamageUnit" (Variables|UnitCombat|GetAttackSpeed) true)))

(event Custom|DamageUnit
  (if (not (Variables|Default|GetDying))
    (bind _asbp_enemy_parent_class (Utilities|Casting|CastToBP_EnemyParentClass (Variables|UnitCombat|GetUnitInRange)))
    (Utilities|IsValid _asbp_enemy_parent_class
      (:Is%20Valid
        (Utilities|FlowControl|FlipFlop
          (:A
            (Components|Animation|PlayAnimation (Variables|Character|GetMesh) (Variables|Default|GetAttackAnim) false))
          (:B
            (Components|Animation|PlayAnimation (Variables|Character|GetMesh) (Variables|Default|GetAttackAnim2) false)))
        (Components|Activation|SetActive (Variables|Default|GetParticleSystem) true true)
        (Default|UnitDamage _asbp_enemy_parent_class (Variables|UnitCombat|GetUnitDamage))
        (Utilities|IsValid (Variables|UnitCombat|GetUnitInRange)
          (:Is%20Valid
            (Utilities|Time|SetTimerbyFunctionName 0 "DamageUnit" (Variables|UnitCombat|GetAttackSpeed))))))))

(event Custom|IsSelected
  (params (IsSelected :type Boolean))
  (Rendering|SetVisibility (Variables|Default|GetSelectionDecal) IsSelected false))

(event EventUnitMove
  (params (Location :type Vector :default "0, 0, 0"))
  (bind _self self)
  (bind _returnvalue (AI|GetAIController _self))
  (Utilities|IsValid _returnvalue
    (:Is%20Valid
      (AI|Navigation|StopMovement _returnvalue)
      (AI|AIMoveTo _returnvalue Location 0 -1.0 "Default" "Default" true true
        (:then
          (Variables|UnitCombat|SetUnitInRange 0)
          (Components|Animation|PlayAnimation (Variables|Character|GetMesh) (Variables|Default|GetWalk) true))
        (:OnRequestFailed
          (bind _aspc_rts (Utilities|Casting|CastToPC_RTS (Game|GetPlayerController 0) :!label _label))
          (for _array_element (Variables|/Game/Blueprints/Player/PC_RTS.PC_RTS_C|GetUnitFormationPositions _aspc_rts)
            (if (< (Math|Vector|Distance(Vector) _array_element (Transformation|GetActorLocation)) (Variables|Default|GetDistanceToClosestForamtionPosition))
              (Variables|Default|SetDistanceToClosestForamtionPosition (Math|Vector|Distance(Vector) _array_element (Transformation|GetActorLocation)))
              (Variables|Default|SetClosestFormationPosition _array_element)))
          (Utilities|Array|RemoveItem (Variables|/Game/Blueprints/Player/PC_RTS.PC_RTS_C|GetUnitFormationPositions _aspc_rts) (Variables|Default|GetClosestFormationPosition))
          (Variables|Default|SetDistanceToClosestForamtionPosition 999999.0)
          (AI|AIMoveTo (AI|GetAIController self) (Variables|Default|GetClosestFormationPosition) 0 -1.0 "Default" "Default" true true
            (:then
              (Components|Animation|PlayAnimation (Variables|Character|GetMesh) (Variables|Default|GetWalk) true))
            (:OnRequestFailed
              (Components|Animation|PlayAnimation (Variables|Character|GetMesh) (Variables|Default|GetIdle) true :!label _label_2)
              (goto _label))
            (:OnMoveFinished
              (goto _label_2))))
        (:OnMoveFinished
          (Components|Animation|PlayAnimation (Variables|Character|GetMesh) (Variables|Default|GetIdle) true))))))

(event EventBeginPlay
  (Utilities|FlowControl|Sequence
    (:then_0
      (CallFunction|UpdateUnitHealthBar))
    (:then_1
      (bind _aspc_rts (Utilities|Casting|CastToPC_RTS (Game|GetPlayerController 0)))
      (Variables|Default|SetAs%20RTS_Controller _aspc_rts)
      (Variables|Default|SetUnitFrameWidget (UserInterface|GetUserWidgetObject (Variables|Default|GetUnitFrame))))
    (:then_2
      (bind _returnvalue (Rendering|Material|CreateDynamicMaterialInstance 0 "None" "None" :!class /Script/Engine.KismetMaterialLibrary))
      (Variables|Default|SetFogOfWarMaterial _returnvalue)
      (bind _returnvalue_2 (Rendering|Material|CreateDynamicMaterialInstance 0 "None" "None" :!class /Script/Engine.KismetMaterialLibrary))
      (Variables|Default|SetFogOfWarRevealMaterial _returnvalue_2))
    (:then_3
      (CallFunction|UpdateUnitHealthBar))))

(event EventAttackUnit
  (params (UnitToAttack :type Actor%20Object%20Reference))
  (bind _self self)
  (bind _returnvalue (AI|GetAIController _self))
  ;[1 1 1] Set Unit location to move to and set unit to attack
  (Variables|UnitCombat|SetUnitInRange UnitToAttack)
  (Utilities|IsValid _returnvalue
    (:Is%20Valid
      (AI|Navigation|StopMovement _returnvalue)
      (AI|AIMoveTo _returnvalue (Math|Vector|MakeVector 0.0 0.0 0.0) UnitToAttack (- (Variables|UnitCombat|GetUnitRange) 5.0) "Default" "Default" true true
        (:then
          (Transformation|SetActorRotation (Math|Rotator|FindLookatRotation (Transformation|GetActorLocation self) (Transformation|GetActorLocation (Variables|UnitCombat|GetUnitInRange))))
          (Components|Animation|PlayAnimation (Variables|Character|GetMesh) (Variables|Default|GetWalk) false))))))

(event EventSelectThis
  ;[1 1 1] Set the Selection Decal
  (Rendering|SetVisibility (Variables|Default|GetSelectionDecal) true false))

(event EventDeselectThis
  ;[1 1 1] Set the Selection Decal
  (Rendering|SetVisibility (Variables|Default|GetSelectionDecal) false false))

(event EventTick
  (params (DeltaSeconds :type Float%20%28single-precision%29))
  (bind _self self)
  (bind _unitinrange (Variables|UnitCombat|GetUnitInRange))
  (bind _returnvalue (Transformation|GetActorLocation _unitinrange))
  (bind _returnvalue_2 (Transformation|GetActorLocation _self))
  (bind _returnvalue_3 (Math|Rotator|FindLookatRotation _returnvalue_2 _returnvalue))
  (Utilities|FlowControl|Sequence
    (:then_0
      ;[1 1 1] Check if unit is available and rotate to look at
      (Utilities|IsValid (Variables|UnitCombat|GetUnitInRange)
        (:Is%20Valid
          (Transformation|SetActorRotation (Math|Rotator|MakeRotator (.roll _returnvalue_3) 0.0 (.yaw _returnvalue_3))))))
    (:then_1
      (CallFunction|OrientHealthtoCamera))))

(event MouseInput|EventActorOnClicked
  (params (ButtonPressed :type Key%20Structure :default "None"))
  (if (== ButtonPressed "LeftMouseButton")
    (bind _aspc_rts (Utilities|Casting|CastToPC_RTS (Game|GetPlayerController 0)))
    (Default|ClearUnitSelection _aspc_rts)
    (if (Rendering|IsVisible (Variables|Default|GetSelectionDecal))
      (Default|RemoveUnitfromSelection _aspc_rts self)
      (else
        (Default|AddUnittoSelection _aspc_rts self)))))

(fn ConstructionScript)

(fn UnitDamaged
  (params (Damage :type Float%20%28double-precision%29))
  ;[1 1 1] Sets Damage
  (bind _output_get (LocalVariables|SetDamageLocal Damage))
  ;[1 1 1] Sets health
  (Variables|UnitCombat|SetCurrentHealth (- (Variables|UnitCombat|GetCurrentHealth) _output_get))
  ;[1 1 1] Is Unit Dead
  (if (<= (Variables|UnitCombat|GetCurrentHealth) 0.0)
    (Actor|DestroyActor)
    (else
      (CallFunction|UpdateUnitHealthBar)))
  (return))

(fn UpdateUnitHealthBar
  (bind _unithealthbar (Variables|Default|GetUnitHealthBar))
  (bind _maxhealth (Variables|UnitCombat|GetMaxHealth))
  (bind _currenthealth (Variables|UnitCombat|GetCurrentHealth))
  (bind _returnvalue (UserInterface|GetUserWidgetObject _unithealthbar))
  (bind _returnvalue_2 (/ _currenthealth _maxhealth))
  (bind _aswb_unit_health_bar (Utilities|Casting|CastToWB_UnitHealthBar _returnvalue))
  (Utilities|IsValid _aswb_unit_health_bar
    (:Is%20Valid
      (Progress|SetPercent (Variables|/Game/Blueprints/Units/WB_UnitHealthBar.WB_UnitHealthBar_C|GetHealthProgBar _aswb_unit_health_bar) _returnvalue_2)
      (if (== _returnvalue_2 1.0)
        (Rendering|SetVisibility (Variables|Default|GetUnitHealthBar) false false)
        (else
          (Rendering|SetVisibility (Variables|Default|GetUnitHealthBar) true false))))
    (:Is%20Not%20Valid
      _))
  (return))

(fn OrientHealthtoCamera
  (bind _returnvalue (Game|GetPlayerCameraManager 0))
  (bind _unithealthbar (Variables|Default|GetUnitHealthBar))
  (bind _unithealthbar_2 (Variables|Default|GetUnitHealthBar))
  (bind _returnvalue_2 (Transformation|GetWorldLocation _unithealthbar_2))
  (bind _transformcomponent (Variables|/Script/Engine.PlayerCameraManager|GetTransformComponent _returnvalue))
  (bind _returnvalue_3 (Transformation|GetWorldLocation _transformcomponent))
  (bind _returnvalue_4 (Math|Rotator|FindLookatRotation _returnvalue_2 _returnvalue_3))
  (bind _returnvalue_5 (Math|Rotator|MakeRotator (.roll _returnvalue_4) (.pitch _returnvalue_4) (.yaw _returnvalue_4)))
  (Utilities|IsValid _unithealthbar
    (:Is%20Valid
      (Transformation|SetWorldRotation _unithealthbar (Math|Rotator|MakeRotator (.roll _returnvalue_5) (.pitch _returnvalue_5) 1.8e+02) false false)
      (return))))

(fn UpdateUnitFrame)

(fn GetSelectedUnits
  (return 0))

(fn GetTeam
  (return (Variables|Details|GetTeamNumber)))

(fn IncremenetWoodAmount
  (return 0))

(fn IncrementFoodAmount
  (return 0))

(fn IncrementMineralAmount
  (return 0))

(fn IsonMyTeam?
  (params (TeamNumber :type Integer))
  (return false))