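; RTS worker unit that gathers Alloy, Mineral or Food from a resource node and delivers it for player resources.
; Assignment caches the closest base, storage or outpost, and AI moves cycle the worker between node and drop-off.
; Node overlap requests collection, and a timer damages the node when done, with multicast effects and a progress bar.
; Major resources collect faster without the bar and set per-area check flags in the game instance.
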(event OnComponentBeginOverlap(Box)
  (params (OverlappedComponent :type Primitive%20Component%20Object%20Reference) (OtherActor :type Actor%20Object%20Reference) (OtherComp :type Primitive%20Component%20Object%20Reference) (OtherBodyIndex :type Integer) (bFromSweep :type Boolean) (SweepResult :type Hit%20Result%20Structure%20%28by%20ref%29))
  (bind _resourcenode (Variables|Default|GetResourceNode))
  (if (== OtherActor _resourcenode)
    (bind _asbp_resource_node (Utilities|Casting|CastToBP_ResourceNode _resourcenode))
    (Default|StartCollect _asbp_resource_node self)))

(event Custom|ResourceCollected
  (Animation|StopAnimMontage (Variables|Default|GetMiningAnim))
  (Variables|Default|SetCollecting false)
  (Rendering|SetVisibility (Variables|Default|GetUnitHealthBar) true false)
  (Utilities|Time|ClearandInvalidateTimerbyHandle (Variables|Default|GetResourceCollectTimer))
  (Variables|Default|SetHasResource? true)
  (CallFunction|WorkerDropoffMove)
  (Game|Damage|ApplyDamage (Variables|Default|GetResourceNode) 1.0 0 0)
  (CallFunction|MulticastStopCollecting)
  (if (Utilities|Enum|Equal(Enum) (Variables|Default|GetResourceName) "NewEnumerator3")
    (switch name (Variables|Default|GetArea)
      (:Beach
        (bind _asbp_artemis_frontier_game_instance (Utilities|Casting|CastToBP_ArtemisFrontierGameInstance (Game|GetGameInstance)))
        (Variables|/Game/Blueprints/BP_ArtemisFrontierGameInstance.BP_ArtemisFrontierGameInstance_C|SetBeachCheck _asbp_artemis_frontier_game_instance true))
      (:Forest
        (bind _asbp_artemis_frontier_game_instance_2 (Utilities|Casting|CastToBP_ArtemisFrontierGameInstance (Game|GetGameInstance)))
        (Variables|/Game/Blueprints/BP_ArtemisFrontierGameInstance.BP_ArtemisFrontierGameInstance_C|SetForestCheck _asbp_artemis_frontier_game_instance_2 true))
      (:Volcano
        (bind _asbp_artemis_frontier_game_instance_3 (Utilities|Casting|CastToBP_ArtemisFrontierGameInstance (Game|GetGameInstance)))
        (Variables|/Game/Blueprints/BP_ArtemisFrontierGameInstance.BP_ArtemisFrontierGameInstance_C|SetVolancoCheck _asbp_artemis_frontier_game_instance_3 true))
      (:Snowy
        (bind _asbp_artemis_frontier_game_instance_4 (Utilities|Casting|CastToBP_ArtemisFrontierGameInstance (Game|GetGameInstance)))
        (Variables|/Game/Blueprints/BP_ArtemisFrontierGameInstance.BP_ArtemisFrontierGameInstance_C|SetSnowyCheck _asbp_artemis_frontier_game_instance_4 true)))))

(event Custom|MulticastStartCollecting
  (bind _particlesystem_0 (Variables|Default|GetParticleSystem_0))
  (bind _particlesystem_0_2 (Variables|Default|GetParticleSystem_0))
  (bind _particlesystem_0_3 (Variables|Default|GetParticleSystem_0))
  ;[1 1 1] multicast start collecting
  (switch Utilities|FlowControl|Switch|SwitchonEResource (Variables|Default|GetResourceName)
    (:NewEnumerator0
      (Effects|Components|ParticleSystem|SetTemplate _particlesystem_0 "/Game/ImportedAssets/Realistic_Starter_VFX_Pack_Vol2/Particles/Destruction/P_Destruction_Wood.P_Destruction_Wood")
      (Components|Activation|SetActive _particlesystem_0 true true))
    (:NewEnumerator1
      (Effects|Components|ParticleSystem|SetTemplate _particlesystem_0_2 "/Game/ImportedAssets/Realistic_Starter_VFX_Pack_Vol2/Particles/Destruction/P_Destruction_Glass.P_Destruction_Glass")
      (Components|Activation|SetActive _particlesystem_0_2 true true))
    (:NewEnumerator2
      (Effects|Components|ParticleSystem|SetTemplate _particlesystem_0_3 "/Game/ImportedAssets/Realistic_Starter_VFX_Pack_Vol2/Particles/Hit/P_Vegetation.P_Vegetation")
      (Components|Activation|SetActive _particlesystem_0_3 true true))))

(event Custom|MulticastStopCollecting
  ;[1 1 1] multicast done collecting
  (Components|Activation|SetActive (Variables|Default|GetParticleSystem_0) false false)
  (Audio|Components|Audio|Stop (Variables|Default|GetAudio)))

(event Custom|MulticastDropOff
  ;[1 1 1] multicast dropoff
)

(event Custom|MulticastUnitNotWorking
  ;[1 1 1] Multicast unit not working
  (Components|Activation|SetActive (Variables|Default|GetParticleSystem_0) false false)
  (Audio|Components|Audio|Stop (Variables|Default|GetAudio)))

(event Custom|WorkerDropoffMove
  (bind _self self)
  (bind _returnvalue (AI|GetAIController _self))
  (Utilities|IsValid _returnvalue
    (:Is%20Valid
      (AI|Navigation|StopMovement _returnvalue)
      (AI|AIMoveTo _returnvalue "0, 0, 0" (Variables|Default|GetDropOffBuilding) -1.0 "Default" "Default" true false false "Default" "Disable"
        (:then
          (Components|Animation|PlayAnimation (Variables|Character|GetMesh) (Variables|Default|GetWalk) true))
        (:OnRequestFailed
          (Components|Animation|PlayAnimation (Variables|Character|GetMesh) (Variables|Default|GetIdle) true :!label _label))
        (:OnMoveFinished
          (goto _label)))
      (Transformation|SetActorRotation (Math|Rotator|FindLookatRotation (Transformation|GetActorLocation) (Transformation|GetActorLocation (Variables|Default|GetDropOffBuilding)))))))

(event Custom|WorkersSoundPlay
  (switch Utilities|FlowControl|Switch|SwitchonEResource (Variables|Default|GetResourceName)
    (:NewEnumerator0
      (Audio|Components|Audio|Play (Variables|Default|GetAudio) 0.0))
    (:NewEnumerator1
      (Audio|Components|Audio|Play (Variables|Default|GetAudio) 0.0))
    (:NewEnumerator2
      (Audio|Components|Audio|Play (Variables|Default|GetAudio) 0.0))))

(event Custom|WorkerMove
  (bind _self self)
  (bind _resourcenode (Variables|Default|GetResourceNode))
  (bind _returnvalue (AI|GetAIController _self))
  (if (and (Utilities|IsValid _returnvalue) (Utilities|IsValid _resourcenode))
    (AI|Navigation|StopMovement _returnvalue)
    (AI|AIMoveTo _returnvalue "0, 0, 0" _resourcenode -1.0 "Default" "Default" true false false "Default" "Disable"
      (:then
        (Components|Animation|PlayAnimation (Variables|Character|GetMesh) (Variables|Default|GetWalk) true))
      (:OnRequestFailed
        (Components|Animation|PlayAnimation (Variables|Character|GetMesh) (Variables|Default|GetIdle) true :!label _label))
      (:OnMoveFinished
        (goto _label)))
    (Transformation|SetActorRotation (Math|Rotator|FindLookatRotation (Transformation|GetActorLocation) (Transformation|GetActorLocation (Variables|Default|GetResourceNode))))))

(event EventTick
  (params (DeltaSeconds :type Float%20%28single-precision%29))
  (if (Variables|Default|GetCollecting)
    (CallFunction|UnitProgress)
    (else
      (Rendering|SetVisibility (Variables|Default|GetProgressBar) false false))))

(event EventBeginPlay
  (Rendering|SetVisibility (Variables|Default|GetProgressBar) false false))

(event EventSetisWorking
  (params (ResourceNode :type Actor%20Object%20Reference))
  (bind _dropoffarray (Variables|Default|GetDropOffArray))
  (Utilities|Array|Clear (Variables|Default|GetDropOffArray))
  (bind _asbp_resource_node (Utilities|Casting|CastToBP_ResourceNode ResourceNode))
  (Variables|Default|SetArea (Variables|/Game/Blueprints/Resources/BP_ResourceNode.BP_ResourceNode_C|GetArea _asbp_resource_node))
  (Variables|Default|SetResourceName (Variables|/Game/Blueprints/Resources/BP_ResourceNode.BP_ResourceNode_C|GetResourceType _asbp_resource_node))
  (Variables|Default|SetIsWorking? true)
  (Variables|Default|SetResourceNode ResourceNode)
  ;[1 1 1] Change for dropoff point
  (Utilities|FlowControl|Sequence
    (:then_0
      (bind _outactors (Actor|GetAllActorsOfClass "/Game/Blueprints/Buildings/UnitBuildingBase.UnitBuildingBase_C"))
      (for _array_element _outactors
        (Utilities|Array|Add _dropoffarray _array_element)))
    (:then_1
      (bind _outactors_2 (Actor|GetAllActorsOfClass "/Game/Blueprints/Buildings/UnitBuildingStorage.UnitBuildingStorage_C"))
      (for _array_element_2 _outactors_2
        (Utilities|Array|Add _dropoffarray _array_element_2)))
    (:then_2
      (bind _outactors_3 (Actor|GetAllActorsOfClass "/Game/Blueprints/Buildings/BP_WorldMapOutpost.BP_WorldMapOutpost_C"))
      (for _array_element_3 _outactors_3
        (Utilities|Array|Add _dropoffarray _array_element_3))
      (for _array_element_4 (Variables|Default|GetDropOffArray)
        ;[1 1 1] Find Closest dropoff building
        (if (< (Transformation|GetDistanceTo _array_element_4 (Variables|Default|GetResourceNode)) (Variables|Default|GetClosestDropOff))
          (Variables|Default|SetDropOffBuilding _array_element_4)
          (Variables|Default|SetClosestDropOff (Transformation|GetDistanceTo _array_element_4 (Variables|Default|GetResourceNode)))))
      (if (Variables|Default|GetHasResource?)
        ;[1 1 1] Move to dropoff
        (CallFunction|WorkerDropoffMove)
        (else
          ;[1 1 1] move to resource
          (CallFunction|WorkerMove))))))

(event EventSetNotWorking
  (Variables|Default|SetIsWorking? false)
  (Utilities|Time|ClearandInvalidateTimerbyHandle (Variables|Default|GetResourceCollectTimer))
  (CallFunction|MulticastUnitNotWorking))

(event EventCollect
  (if (Variables|Default|GetIsWorking?)
    (if (Variables|Default|GetHasResource?)
      ;[1 1 1] has resource, move to dropoff
      (CallFunction|WorkerDropoffMove)
      (elif (not (Utilities|Time|IsValidTimerHandle (Variables|Default|GetResourceCollectTimer)))
        ;[1 1 1] stop movement
        (CallFunction|UnitMove (Transformation|GetActorLocation))
        (if (not (Utilities|Enum|Equal(Enum) (Variables|Default|GetResourceName) "NewEnumerator3"))
          (CallFunction|MulticastStartCollecting)
          (CallFunction|WorkersSoundPlay)
          (bind _returnvalue (Utilities|Time|SetTimerbyEvent (delegate Custom|ResourceCollected) 4.0))
          (Variables|Default|SetResourceCollectTimer _returnvalue)
          (Variables|Default|SetCollecting true)
          (Components|Animation|PlayAnimation (Variables|Character|GetMesh) (Variables|Default|GetMiningAnim) true)
          (Utilities|FlowControl|RetriggerableDelay 4.0)
          (CallFunction|MulticastStartCollecting)
          (else
            (CallFunction|MulticastStartCollecting)
            (CallFunction|WorkersSoundPlay)
            (bind _returnvalue_2 (Utilities|Time|SetTimerbyEvent (delegate Custom|ResourceCollected) 2.0))
            (Variables|Default|SetResourceCollectTimer _returnvalue_2)
            (Utilities|FlowControl|RetriggerableDelay 4.0)
            (CallFunction|MulticastStartCollecting)))))))

(event EventDropoff
  (if (Variables|Default|GetIsWorking?)
    (if (Variables|Default|GetHasResource?)
      (Class|BPIInterface|IncrementResourceAmount(Message) (Game|GetPlayerController 0) 10 (Variables|Default|GetResourceName))
      (Variables|Default|SetHasResource? false)
      (CallFunction|MulticastDropOff)
      (CallFunction|WorkerMove)
      (else
        ;[1 1 1] Move to resource, if no resource
        (CallFunction|WorkerMove)))))

(fn ConstructionScript
  (|CallParentFunction)
  (Utilities|Array|Add (Variables|Default|GetMeshForColouring) 0))

(fn IsonMyTeam?
  (params (TeamNumber :type Integer))
  (return false))

(fn UnitProgress
  (bind _returnvalue (Game|GetPlayerCameraManager 0))
  (bind _progressbar (Variables|Default|GetProgressBar))
  (bind _progressbar_2 (Variables|Default|GetProgressBar))
  (bind _returnvalue_2 (UserInterface|GetUserWidgetObject _progressbar))
  (bind _returnvalue_3 (Transformation|GetWorldLocation _progressbar_2))
  (bind _transformcomponent (Variables|/Script/Engine.PlayerCameraManager|GetTransformComponent _returnvalue))
  (bind _returnvalue_4 (Transformation|GetWorldLocation _transformcomponent))
  (bind _asprogress_bar (Utilities|Casting|CastToProgressBar _returnvalue_2))
  (bind _returnvalue_5 (Math|Rotator|FindLookatRotation _returnvalue_3 _returnvalue_4))
  (bind _returnvalue_6 (Math|Rotator|MakeRotator (.roll _returnvalue_5) (.pitch _returnvalue_5) (.yaw _returnvalue_5)))
  (Rendering|SetVisibility (Variables|Default|GetUnitHealthBar) false false)
  (Utilities|IsValid _asprogress_bar
    (:Is%20Valid
      (Progress|SetPercent (Variables|/Game/UI/ProgressBar.ProgressBar_C|GetProgressBar_19 _asprogress_bar) (/ (Class|KismetSystemLibrary|GetTimerElapsedTimeHandle (Variables|Default|GetResourceCollectTimer)) 4.0))
      (Rendering|SetVisibility (Variables|Default|GetProgressBar) true false)
      (Transformation|SetWorldRotation (Variables|Default|GetProgressBar) (Math|Rotator|MakeRotator (.roll _returnvalue_6) (.pitch _returnvalue_6) 1.8e+02) false false)
      (return))
    (:Is%20Not%20Valid
      (return))))