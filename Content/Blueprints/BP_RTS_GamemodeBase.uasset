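; RTS game mode base that places each joining player at a random start camp and maintains the fog of war reveal target.
; The construction script gathers all player start camps into a pool.
; Each new player possesses a camera pawn spawned at a camp drawn from that pool, receives its camp, incrementing team number and team colour, and the camp is removed.
; Tick clears the fog of war reveal render target to black every frame.
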(event EventTick
  (params (DeltaSeconds :type Float%20%28single-precision%29))
  (Rendering|ClearRenderTarget2D "/Game/FogOfWar/Materials/FogOfWarRevealRender.FogOfWarRevealRender"))

(event EventHandleStartingNewPlayer
  (params (NewPlayer :type Player%20Controller%20Object%20Reference))
  (Variables|Default|SetSelectedStartCamp (.OutItem (Utilities|Array|Random (Variables|Default|GetStart%20Camps))))
  (bind _returnvalue (Game|SpawnActorfromClass "/Game/Blueprints/Player/BP_CameraP.BP_CameraP_C" (Transformation|GetWorldTransform (Variables|/Game/Blueprints/BP_PlayerStartCamp.BP_PlayerStartCamp_C|GetCamera%20Location (Variables|Default|GetSelectedStartCamp))) "Undefined" "MultiplyWithRoot" 0 0))
  (Pawn|Possess NewPlayer _returnvalue)
  (Class|BPIInterface|SetupPlayerStart(Message) NewPlayer (Variables|Default|GetSelectedStartCamp) (Variables|Default|GetTeamNumber) (Utilities|Array|Get(acopy) (Variables|Default|GetTeamColour) (Variables|Default|GetTeamNumber)))
  (Math|Integer|IncrementInt (Variables|Default|GetTeamNumber)
    (:%20%20
      (Utilities|Array|RemoveItem (Variables|Default|GetStart%20Camps) (Variables|Default|GetSelectedStartCamp)))))

(fn ConstructionScript
  (bind _outactors (Actor|GetAllActorsOfClass "/Game/Blueprints/BP_PlayerStartCamp.BP_PlayerStartCamp_C"))
  (Variables|Default|SetStart%20Camps _outactors))