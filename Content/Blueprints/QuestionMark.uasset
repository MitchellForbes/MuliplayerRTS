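; QuestionMark is a world marker actor that shows while main quest MQ001 is active.
; It starts hidden and destroys itself on BeginPlay if the game instance reports MQ001 completed.
; Each Tick it polls BP_ArtemisFrontierGameInstance, unhiding when the quest is active and destroying itself once completed.
; The quest ID is hard-coded, and visibility relies on per-frame polling rather than quest events.
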(event EventBeginPlay
  (Rendering|SetActorHiddenInGame true)
  (bind _asbp_artemis_frontier_game_instance (Utilities|Casting|CastToBP_ArtemisFrontierGameInstance (Game|GetGameInstance)))
  (if (.ReturnValue (Default|QueryCompletedQuests _asbp_artemis_frontier_game_instance "MQ001"))
    (Actor|DestroyActor)))

(event EventTick
  (params (DeltaSeconds :type Float%20%28single-precision%29))
  (Utilities|FlowControl|Sequence
    (:then_0
      (bind _asbp_artemis_frontier_game_instance (Utilities|Casting|CastToBP_ArtemisFrontierGameInstance (Game|GetGameInstance)))
      (if (Default|QueryActiveQuest _asbp_artemis_frontier_game_instance "MQ001")
        (Rendering|SetActorHiddenInGame false)))
    (:then_1
      (bind _asbp_artemis_frontier_game_instance_2 (Utilities|Casting|CastToBP_ArtemisFrontierGameInstance (Game|GetGameInstance)))
      (if (.ReturnValue (Default|QueryCompletedQuests _asbp_artemis_frontier_game_instance_2 "MQ001"))
        (Actor|DestroyActor)))))

(fn ConstructionScript)