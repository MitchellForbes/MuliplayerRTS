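; Trigger-volume actor that switches the environmental audio track when the player enters its box.
; Tick tests the player pawn against the box bounds whenever its sound differs from the one stored in the Artemis Frontier game instance.
; On entry it stops every BP_AudioSelect, reports the new sound to the game instance and plays from the shared saved position.
; Playback-percent callbacks feed that position back to the game instance.
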(event Custom|OnAudioPlaybackPercent_Event
  (params (PlayingSoundWave :type Sound%20Wave%20Object%20Reference) (PlaybackPercent :type Float%20%28single-precision%29))
  (bind _asbp_artemis_frontier_game_instance (Utilities|Casting|CastToBP_ArtemisFrontierGameInstance (Game|GetGameInstance)))
  (Default|CurrentPositioninAudio _asbp_artemis_frontier_game_instance (* PlaybackPercent (Variables|/Script/Engine.SoundBase|GetDuration PlayingSoundWave))))

(event EventTick
  (params (DeltaSeconds :type Float%20%28single-precision%29))
  (bind _envromentsound (Variables|Default|GetEnvromentSound))
  (bind _box (Variables|Default|GetBox))
  (bind (_origin _boxextent) (Collision|GetComponentBounds _box))
  (bind _asbp_artemis_frontier_game_instance (Utilities|Casting|CastToBP_ArtemisFrontierGameInstance (Game|GetGameInstance)))
  (if (not (== _envromentsound (Variables|/Game/Blueprints/BP_ArtemisFrontierGameInstance.BP_ArtemisFrontierGameInstance_C|GetEnviromentalAudio _asbp_artemis_frontier_game_instance)))
    (if (Math|Geometry|IsPointinBox (Transformation|GetActorLocation (Game|Player|GetPlayerPawn 0)) _origin _boxextent)
      (Variables|Default|SetCurrentDuration (Variables|/Game/Blueprints/BP_ArtemisFrontierGameInstance.BP_ArtemisFrontierGameInstance_C|GetCurrentDuration _asbp_artemis_frontier_game_instance))
      (Audio|Components|Audio|SetSound (Variables|Default|GetAudioComponent) _envromentsound)
      (bind _outactors (Actor|GetAllActorsOfClass "BP_AudioSelect_C"))
      (for _array_element _outactors
        (Audio|Components|Audio|Stop (Variables|BP_AudioSelect_C|GetAudioComponent _array_element)))
      (EventDispatchers|BindEventtoOnAudioPlaybackPercent (Variables|Default|GetAudioComponent) (delegate Custom|OnAudioPlaybackPercent_Event))
      (Development|PrintString (Utilities|GetDisplayName (Variables|Default|GetEnvromentSound)))
      (bind _asbp_artemis_frontier_game_instance_2 (Utilities|Casting|CastToBP_ArtemisFrontierGameInstance (Game|GetGameInstance)))
      (Default|PlayEnviromentalSounds _asbp_artemis_frontier_game_instance_2 (Variables|Default|GetEnvromentSound))
      (Audio|Components|Audio|Play (Variables|Default|GetAudioComponent) (Variables|Default|GetCurrentDuration)))))

(event EventBeginPlay
  (Audio|Components|Audio|SetSound (Variables|Default|GetAudioComponent) (Variables|Default|GetEnvromentSound)))

(fn ConstructionScript)