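; Game instance for Artemis Frontier that manages quests and per-level saves.
; Quests run as spawned Quest_Base actors, rebuilt from active IDs and a saved stage/progress map, with a tracker widget.
; Resource and building updates substring-match data table objective IDs, then report progress.
; Actors tagged SaveLocation are stored by class and transform in a level-named save and respawned on load; SaveUnitLocation writes the slot before copying in new arrays.
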(event Custom|ReloadQuestData
  (Utilities|Array|Clear (Variables|Quests|GetCurrentQuests))
  (bind _outactors (Actor|GetAllActorsOfClass "/Game/QuestSystem/Blueprints/Quest_Base.Quest_Base_C"))
  (if (Utilities|Array|IsValidIndex _outactors)
    (for _array_element _outactors
      (Actor|DestroyActor _array_element)))
  (for _array_element_2 (Variables|Quests|GetCurrentActiveQuests)
    (bind _returnvalue (Quests|AddNewQuest _array_element_2))
    (Variables|/Game/QuestSystem/Blueprints/Quest_Base.Quest_Base_C|SetCurrentStage _returnvalue (.CurrentStage (Utilities|Struct|BreakStruct_FSaveQuestData (.Value (Utilities|Map|Find (Variables|Quests|GetQuestProgress) _array_element_2)))))
    (Variables|/Game/QuestSystem/Blueprints/Quest_Base.Quest_Base_C|SetCurrentObjectiveProgress _returnvalue (.Progress (Utilities|Struct|BreakStruct_FSaveQuestData (.Value (Utilities|Map|Find (Variables|Quests|GetQuestProgress) _array_element_2)))))))

(event Custom|PlayEnviromentalSounds
  (params (Enviroment%20Sound :type Sound%20Wave%20Object%20Reference))
  (Variables|Default|SetEnviromentalAudio Enviroment%20Sound))

(event Custom|CurrentPositionInAudio
  (params (CurrentDuration :type Float%20%28double-precision%29))
  (Variables|Default|SetCurrentDuration CurrentDuration))

(event EventInit
  (Variables|Quests|SetQuestData "/Game/QuestSystem/EnumsDataTables/QuestData.QuestData")
  (SaveLevel|InitLevelSaveData)
  (Rendering|ClearRenderTarget2D 0)
  (Rendering|ClearRenderTarget2D 0))

(fn AddNewQuest
  (params (QuestID :type Name))
  (Utilities|Array|AddUnique (Variables|Quests|GetCurrentActiveQuests) QuestID)
  (bind _returnvalue (Game|SpawnActorfromClass "/Game/QuestSystem/Blueprints/Quest_Base.Quest_Base_C" (Math|Transform|MakeTransform "0, 0, 0" "0, 0, 0" "1.000000,1.000000,1.000000") "Undefined" "MultiplyWithRoot" 0 QuestID 0))
  (Variables|/Game/QuestSystem/Blueprints/Quest_Base.Quest_Base_C|SetCurrentStage _returnvalue 0)
  (Utilities|Array|Add (Variables|Quests|GetCurrentQuests) _returnvalue)
  (return _returnvalue))

(fn CompleteQuest
  (params (QuestID :type Name))
  (Development|PrintString "Hello")
  (Utilities|Array|AddUnique (Variables|Quests|GetCompletedQuests) QuestID)
  (Utilities|Array|RemoveItem (Variables|Quests|GetCurrentActiveQuests) QuestID)
  (bind _array_element (Quests|GetQuestActor QuestID))
  (Variables|/Game/QuestSystem/Blueprints/Quest_Base.Quest_Base_C|SetIsTurnedIn? _array_element true)
  (Utilities|Array|RemoveItem (Variables|Quests|GetCurrentQuests) _array_element)
  (Actor|DestroyActor _array_element)
  (Audio|PlaySound2D "/Game/Audio/UISounds/Instrument/PLAYER_ACHIEVE_3.PLAYER_ACHIEVE_3" 1.0 1.0 0.0 0 0)
  (Default|CallOnQuestCompleted _array_element))

(fn QueryActiveQuest
  (params (QuestID :type Name))
  (return (Utilities|Array|ContainsItem (Variables|Quests|GetCurrentActiveQuests) QuestID)))

(fn TrackQuest
  (params (QuestActor :type Quest%20Base%20Object%20Reference))
  (bind _tracker (Variables|Quests|GetTracker)
    (:then
      (Default|Update _tracker QuestActor))
    (:else
      (bind _returnvalue (UserInterface|CreateWidget "/Game/QuestSystem/Widgets/W_Tracker.W_Tracker_C" 0 QuestActor))
      (bind _output_get (Variables|Quests|SetTracker _returnvalue))
      (UserInterface|Viewport|AddtoViewport _output_get -1))))

(fn GetQuestActor
  (params (QuestID :type Name))
  (for _array_element (Variables|Quests|GetCurrentQuests)
    (Utilities|IsValid _array_element
      (:Is%20Valid
        (if (== (Variables|/Game/QuestSystem/Blueprints/Quest_Base.Quest_Base_C|GetQuestID _array_element) QuestID)
          (return _array_element))))))

(fn TurninQuest
  (params (QuestID :type Name))
  (Utilities|FlowControl|Sequence
    (:then_0
      (bind _array_element (Quests|GetQuestActor QuestID)))
    (:then_1
      (Quests|CompleteQuest QuestID))))

(fn QueryCompletedQuests
  (params (QuestID :type Name))
  (bind _completedquests (Variables|Quests|GetCompletedQuests))
  (bind _returnvalue (Utilities|Array|ContainsItem _completedquests QuestID))
  (bind _array_element (Quests|GetQuestActor QuestID))
  (Utilities|IsValid _array_element
    (:Is%20Valid
      (return _returnvalue (Variables|/Game/QuestSystem/Blueprints/Quest_Base.Quest_Base_C|GetIsTurnedIn? _array_element)))
    (:Is%20Not%20Valid
      (return _returnvalue true))))

(fn SaveQuestDetails
  (for _array_element (Variables|Quests|GetCurrentQuests)
    (Utilities|Map|Add (Variables|Quests|GetQuestProgress) (Variables|/Game/QuestSystem/Blueprints/Quest_Base.Quest_Base_C|GetQuestID _array_element) (Utilities|Struct|MakeStruct_FSaveQuestData (Variables|/Game/QuestSystem/Blueprints/Quest_Base.Quest_Base_C|GetCurrentObjectiveProgress _array_element) (Variables|/Game/QuestSystem/Blueprints/Quest_Base.Quest_Base_C|GetCurrentStage _array_element)))))

(fn UpdateCollectionQuests
  (for _array_element (Variables|Quests|GetCurrentActiveQuests)
    (bind _returnvalue (Utilities|GetDataTableRow "/Game/QuestSystem/EnumsDataTables/QuestData.QuestData" _array_element)
      (:then
        (for (_ _array_index) (.Objectives (Utilities|Struct|BreakStruct_FStageDetails (Utilities|Array|Get(acopy) (.Stages (Utilities|Struct|BreakStruct_FQuestDetails _returnvalue)))))
          (if (Utilities|Enum|Equal(Enum) (.Type (Utilities|Struct|BreakStruct_FObjectiveDetails (Utilities|Array|Get(acopy) (.Objectives (Utilities|Struct|BreakStruct_FStageDetails (Utilities|Array|Get(acopy) (.Stages (Utilities|Struct|BreakStruct_FQuestDetails _returnvalue))))) _array_index))) "NewEnumerator3")
            (for (_ _array_index_2) (Utilities|Array|MakeArray (Variables|Resources|GetResourceWood) (Variables|Resources|GetResourceFood) (Variables|Resources|GetResourceMinerals))
              (LocalVariables|SetArrayIndex _array_index_2)
              (LocalVariables|SetObjectiveId (.ObjectiveID (Utilities|Struct|BreakStruct_FObjectiveDetails (Utilities|Array|Get(acopy) (.Objectives (Utilities|Struct|BreakStruct_FStageDetails (Utilities|Array|Get(acopy) (.Stages (Utilities|Struct|BreakStruct_FQuestDetails _returnvalue))))) _array_index))))
              (switch int _array_index_2
                (:0
                  (if (Utilities|String|Contains (LocalVariables|GetObjectiveId) (Utilities|Array|Get(acopy) (Variables|Resources|GetResourceStringArray) (LocalVariables|GetArrayIndex)) true)
                    (switch string (Utilities|Array|Get(acopy) (Variables|Resources|GetResourceStringArray) (LocalVariables|GetArrayIndex)) :!label _label
                      (:Wood
                        (Default|CallOnObjectiveIDCalled (LocalVariables|GetObjectiveId) (Variables|Resources|GetResourceWood)))
                      (:Food
                        (Default|CallOnObjectiveIDCalled (LocalVariables|GetObjectiveId) (Variables|Resources|GetResourceFood)))
                      (:Mineral
                        (Default|CallOnObjectiveIDCalled (LocalVariables|GetObjectiveId) (Variables|Resources|GetResourceMinerals))))))
                (:1
                  (if (Utilities|String|Contains (LocalVariables|GetObjectiveId) (Utilities|Array|Get(acopy) (Variables|Resources|GetResourceStringArray) (LocalVariables|GetArrayIndex)) true)
                    (goto _label)))
                (:2
                  (if (Utilities|String|Contains (LocalVariables|GetObjectiveId) (Utilities|Array|Get(acopy) (Variables|Resources|GetResourceStringArray) (LocalVariables|GetArrayIndex)) true)
                    (goto _label))))))))))
  (return))

(fn InitLevelSaveData
  (bind _returnvalue (Game|GetCurrentLevelName true))
  (bind _returnvalue_2 (SaveGame|DoesSaveGameExist _returnvalue))
  (if _returnvalue_2
    (bind _returnvalue_3 (Game|GetCurrentLevelName true))
    (bind _returnvalue_4 (SaveGame|LoadGamefromSlot _returnvalue_3))
    (bind _aslevelsave_data (Utilities|Casting|CastToLevelsaveData _returnvalue_4))
    (Variables|SaveLevel|SetLevelSaveObject _aslevelsave_data)
    (else
      (bind _returnvalue_5 (SaveGame|CreateSaveGameObject "/Game/Blueprints/Player/LevelsaveData.LevelsaveData_C"))
      (Variables|SaveLevel|SetLevelSaveObject _returnvalue_5))))

(fn SaveLevelData
  (bind _returnvalue (Game|GetCurrentLevelName true))
  (SaveGame|SaveGametoSlot (Variables|SaveLevel|GetLevelSaveObject) _returnvalue))

(fn SaveUnitLocation
  (bind _outactors (Actor|GetAllActorswithTag "SaveLocation"))
  (Utilities|Array|Clear (Variables|SaveLevel|GetActorClassSave))
  (Utilities|Array|Clear (Variables|SaveLevel|GetActorLocationSave))
  (for _array_element _outactors
    (Utilities|Array|Add (Variables|SaveLevel|GetActorClassSave) (Utilities|GetClass _array_element))
    (Utilities|Array|Add (Variables|SaveLevel|GetActorLocationSave) (Transformation|GetActorTransform _array_element)))
  (SaveLevel|SaveLevelData)
  (Utilities|Array|Clear (Variables|/Game/Blueprints/Player/LevelsaveData.LevelsaveData_C|GetUnits (Variables|SaveLevel|GetLevelSaveObject)))
  (Utilities|Array|Clear (Variables|/Game/Blueprints/Player/LevelsaveData.LevelsaveData_C|GetUnitLocations (Variables|SaveLevel|GetLevelSaveObject)))
  (Variables|/Game/Blueprints/Player/LevelsaveData.LevelsaveData_C|SetUnits (Variables|SaveLevel|GetLevelSaveObject) (Variables|SaveLevel|GetActorClassSave))
  (Variables|/Game/Blueprints/Player/LevelsaveData.LevelsaveData_C|SetUnitLocations (Variables|SaveLevel|GetLevelSaveObject) (Variables|SaveLevel|GetActorLocationSave)))

(fn LoadActorLocation
  (bind _levelsaveobject (Variables|SaveLevel|GetLevelSaveObject))
  (bind _units (Variables|/Game/Blueprints/Player/LevelsaveData.LevelsaveData_C|GetUnits _levelsaveobject))
  (for _array_element _units
    (bind _outactors (Actor|GetAllActorsOfClass _array_element))
    (for _array_element_2 _outactors
      (Actor|DestroyActor _array_element_2)))
  (for (_array_element_3 _array_index) _units
    (bind _returnvalue (Game|SpawnActorfromClass _array_element_3 (Utilities|Array|Get(acopy) (Variables|/Game/Blueprints/Player/LevelsaveData.LevelsaveData_C|GetUnitLocations _levelsaveobject) _array_index) "AdjustIfPossibleButAlwaysSpawn" "MultiplyWithRoot" 0 0))
    (if (Utilities|ClassIsChildOf (Utilities|GetClass _returnvalue) "/Game/Blueprints/Buildings/UnitBuildingBase.UnitBuildingBase_C")
      (bind _asunit_building_base (Utilities|Casting|CastToUnitBuildingBase _returnvalue))
      (Default|SetMeshMaterials _asunit_building_base)
      (Variables|/Game/Blueprints/Buildings/UnitBuildingBase.UnitBuildingBase_C|SetIsActive _asunit_building_base true))))

(fn UpdateBuildingQuest
  (params (BuildingID :type String))
  (LocalVariables|SetBuildID BuildingID)
  (for _array_element (Variables|Quests|GetCurrentActiveQuests)
    ;[1 1 1] Check Quest type
    (bind _returnvalue (Utilities|GetDataTableRow "/Game/QuestSystem/EnumsDataTables/QuestData.QuestData" _array_element)
      (:then
        (for (_ _array_index) (.Stages (Utilities|Struct|BreakStruct_FQuestDetails _returnvalue))
          (for (_ _array_index_2) (.Objectives (Utilities|Struct|BreakStruct_FStageDetails (Utilities|Array|Get(acopy) (.Stages (Utilities|Struct|BreakStruct_FQuestDetails _returnvalue)) _array_index)))
            (if (Utilities|Enum|Equal(Enum) (.Type (Utilities|Struct|BreakStruct_FObjectiveDetails (Utilities|Array|Get(acopy) (.Objectives (Utilities|Struct|BreakStruct_FStageDetails (Utilities|Array|Get(acopy) (.Stages (Utilities|Struct|BreakStruct_FQuestDetails _returnvalue)) _array_index))) _array_index_2))) "NewEnumerator4")
              (if (Utilities|String|Contains (.ObjectiveID (Utilities|Struct|BreakStruct_FObjectiveDetails (Utilities|Array|Get(acopy) (.Objectives (Utilities|Struct|BreakStruct_FStageDetails (Utilities|Array|Get(acopy) (.Stages (Utilities|Struct|BreakStruct_FQuestDetails _returnvalue)) _array_index))) _array_index_2))) (LocalVariables|GetBuildID))
                (Default|CallOnObjectiveIDCalled (.ObjectiveID (Utilities|Struct|BreakStruct_FObjectiveDetails (Utilities|Array|Get(acopy) (.Objectives (Utilities|Struct|BreakStruct_FStageDetails (Utilities|Array|Get(acopy) (.Stages (Utilities|Struct|BreakStruct_FQuestDetails _returnvalue)) _array_index))) _array_index_2))) 1))))))))
  (return))

(fn WritetoTxtTimer)

(fn StartTimer
  (Math|Integer|IncrementInt (Variables|Default|GetSeconds_0)))

(fn UpdateCheck
  (bind _foundwidgets (Widget|GetAllWidgetsOfClass "/Game/UI/W_HUDWorldMap.W_HUDWorldMap_C" true))
  (for _array_element _foundwidgets
    _))