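; BP_FogOfWar is a fog of war actor that covers a rectangular area with a grid of cloud meshes.
; The construction script calls PlaceClouds, which rebuilds the ISMClouds instances from GridSize and Gap, offset from the actor location.
; Each instance gets a random quarter-turn yaw and a random uniform scale to vary the look.
; ClearFog removes a single cloud by instance index.
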(event Custom|PlaceClouds
  (bind _gridsize (Variables|Default|GetGridSize))
  (bind _gap (Variables|Default|GetGap))
  (bind _returnvalue (Utilities|Operators|Divide (.y _gridsize) 2.0 _gap))
  (bind _returnvalue_2 (Utilities|Operators|Divide (.x _gridsize) 2.0 _gap))
  (Components|InstancedStaticMesh|ClearInstances (Variables|Default|GetISM_Clouds))
  (for _index (range (Math|Float|Truncate (* _returnvalue_2 -1.0)) (Math|Float|Truncate _returnvalue_2))
    (for _index_2 (range (Math|Float|Truncate (* _returnvalue -1.0)) (Math|Float|Truncate _returnvalue))
      (Components|InstancedStaticMesh|AddInstance (Variables|Default|GetISM_Clouds) (Math|Transform|MakeTransform (+ (Transformation|GetActorLocation) (Math|Vector|MakeVector (* _index (Variables|Default|GetGap)) (* _index_2 (Variables|Default|GetGap)) 0.0)) (Math|Rotator|MakeRotator 0.0 0.0 (Math|Conversions|ToFloat(Integer) (* (Math|Random|RandomIntegerinRange 0 4) 90))) (Math|Conversions|ToVector(Float) (Math|Random|RandomFloatinRange (Variables|Default|GetMin%20Scale) (Variables|Default|GetMax%20Scale)))) false))))

(event EventClearFog
  (params (Index :type Integer))
  (Class|InstancedStaticMeshComponent|RemoveInstance (Variables|Default|GetISM_Clouds) Index))

(fn ConstructionScript
  (CallFunction|PlaceClouds))