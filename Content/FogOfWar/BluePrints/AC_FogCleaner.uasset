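; AC_FogCleaner is a component that clears fog-of-war clouds around its owning actor.
; A looping one-second timer runs two Camera-channel line traces from just above the owner: one straight up, then one toward the player camera.
; Each hit sends a clear-fog message to the hit actor with the HitItem index, so that actor can clear the specific cloud struck.
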(event Custom|CheckFog
  (bind _returnvalue (Components|GetOwner))
  (bind _returnvalue_2 (Transformation|GetActorLocation _returnvalue))
  (bind _returnvalue_3 (+ _returnvalue_2 "0.000000,0.000000,200.000000"))
  (Utilities|TraceClouds _returnvalue_3 (+ _returnvalue_2 "0.000000,0.000000,10000.000000")
    (:OutputPin
      (Utilities|TraceClouds _returnvalue_3 (Camera|GetCameraLocation (Variables|/Script/Engine.PlayerController|GetPlayerCameraManager (Game|GetPlayerController 0)))))))

(event EventBeginPlay
  (Utilities|Time|SetTimerbyEvent (delegate Custom|CheckFog) 1.0 true))