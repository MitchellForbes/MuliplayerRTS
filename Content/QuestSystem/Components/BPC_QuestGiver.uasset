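; Quest giver component that marks its owner as offering a quest and handles interaction to offer up to two quests with optional prerequisites.
; Tick spawns a BP_Quest marker above the owner once, keeps it following, and destroys it when the quest becomes active.
; InteractWith checks quest state in BP_ArtemisFrontierGameInstance, then auto-accepts, opens W_QuestWindow from data table rows, or returns the owner's name for turn-in.
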(event EventTick
  (params (DeltaSeconds :type Float%20%28single-precision%29))
  (bind _returnvalue (Components|GetOwner))
  (bind _returnvalue_2 (Transformation|GetActorTransform _returnvalue))
  (bind _returnvalue_3 (+ (.z (.location _returnvalue_2)) 75.0))
  (bind _returnvalue_4 (Math|Transform|MakeTransform (Math|Vector|MakeVector (.x (.location _returnvalue_2)) (.y (.location _returnvalue_2)) _returnvalue_3) (.rotation _returnvalue_2) (.scale _returnvalue_2)))
  (if (Variables|Default|GetRequiresPreRec)
    (bind _newparam (CallFunction|PreRecQuests))
    (if _newparam
      (Utilities|FlowControl|Sequence :!label _label
        (:then_0
          (Utilities|FlowControl|DoOnce false
            (:Completed
              (bind _asbp_artemis_frontier_game_instance (Utilities|Casting|CastToBP_ArtemisFrontierGameInstance (Game|GetGameInstance)))
              (for _array_element (Variables|/Game/Blueprints/BP_ArtemisFrontierGameInstance.BP_ArtemisFrontierGameInstance_C|GetCompletedQuests _asbp_artemis_frontier_game_instance)
                (if (== (.rowname (Variables|Default|GetQuestData)) _array_element)
                  (Variables|Default|SetPutUpQuestionMark (== (.rowname (Variables|Default|GetQuestData)) _array_element))))
              (if (not (Variables|Default|GetPutUpQuestionMark))
                (bind _returnvalue_5 (Game|SpawnActorfromClass "/Game/QuestSystem/Blueprints/BP_Quest.BP_Quest_C" _returnvalue_4 "Undefined" "MultiplyWithRoot" 0 0))
                (Variables|Default|SetQuestMark _returnvalue_5)))))
        (:then_1
          (Utilities|IsValid (Variables|Default|GetQuestMark)
            (:Is%20Valid
              (bind _asbp_artemis_frontier_game_instance_2 (Utilities|Casting|CastToBP_ArtemisFrontierGameInstance (Game|GetGameInstance)))
              (for _array_element_2 (Variables|/Game/Blueprints/BP_ArtemisFrontierGameInstance.BP_ArtemisFrontierGameInstance_C|GetCurrentActiveQuests _asbp_artemis_frontier_game_instance_2)
                (if (== _array_element_2 (.rowname (Variables|Default|GetQuestData)))
                  (Actor|DestroyActor (Variables|Default|GetQuestMark)))))))
        (:then_2
          (Utilities|IsValid (Variables|Default|GetQuestMark)
            (:Is%20Valid
              (Transformation|SetActorTransform (Variables|Default|GetQuestMark) _returnvalue_4))))))
    (else
      (goto _label))))

(fn DisplayQuest
  (bind _questdata (Variables|Default|GetQuestData))
  (bind _returnvalue (Utilities|GetDataTableRow (.datatable _questdata) (.rowname _questdata))
    (:then
      (bind _returnvalue_2 (UserInterface|CreateWidget "/Game/QuestSystem/Widgets/W_QuestWindow.W_QuestWindow_C" 0 _returnvalue (.rowname _questdata)))
      (UserInterface|Viewport|AddtoViewport _returnvalue_2 0))))

(fn DisplayRewards
  (bind _questdata (Variables|Default|GetQuestData))
  (bind _returnvalue (Utilities|GetDataTableRow "/Game/QuestSystem/EnumsDataTables/QuestData.QuestData" (.rowname _questdata))
    (:then
      (bind _returnvalue_2 (UserInterface|CreateWidget "/Game/QuestSystem/Widgets/W_QuestRewards.W_QuestRewards_C" 0 _returnvalue (.rowname _questdata)))
      (UserInterface|Viewport|AddtoViewport _returnvalue_2 0))))

(fn IsMainQuest?
  (return (Utilities|String|Contains (Utilities|String|ToString(Name) (.rowname (Variables|Default|GetQuestData))) "MQ")))

(fn QuestBeforeDone
  (LocalVariables|SetQuestString "")
  (for _array_element (Utilities|String|GetCharacterArrayfromString (Utilities|String|ToString(Name) (.rowname (Variables|Default|GetQuestData))))
    (if (Class|KismetStringLibrary|IsNumeric _array_element)
      (LocalVariables|SetQuestString (Utilities|String|Append (LocalVariables|GetQuestString) _array_element))))
  (return))

(fn PreRecQuests
  (if (Variables|Default|GetRequiresPreRec)
    (bind _asbp_artemis_frontier_game_instance (Utilities|Casting|CastToBP_ArtemisFrontierGameInstance (Game|GetGameInstance)))
    (for _array_element (Variables|/Game/Blueprints/BP_ArtemisFrontierGameInstance.BP_ArtemisFrontierGameInstance_C|GetCompletedQuests _asbp_artemis_frontier_game_instance)
      (if (== _array_element (.RowName (Utilities|Struct|BreakDataTableRowHandle (Variables|Default|GetPreRecQuestIsComplete))))
        (return true)))
    (return false)
    (else
      (return true))))

(fn DisplayQuest2
  (bind _secondquest (Variables|Default|GetSecondQuest))
  (bind _returnvalue (Utilities|GetDataTableRow (.datatable _secondquest) (.rowname _secondquest))
    (:then
      (bind _returnvalue_2 (UserInterface|CreateWidget "/Game/QuestSystem/Widgets/W_QuestWindow.W_QuestWindow_C" 0 _returnvalue (.rowname _secondquest)))
      (UserInterface|Viewport|AddtoViewport _returnvalue_2 0))))

(fn PreRecQuests2
  (if (Variables|Default|GetRequiresPreRec)
    (bind _asbp_artemis_frontier_game_instance (Utilities|Casting|CastToBP_ArtemisFrontierGameInstance (Game|GetGameInstance)))
    (for _array_element (Variables|/Game/Blueprints/BP_ArtemisFrontierGameInstance.BP_ArtemisFrontierGameInstance_C|GetCompletedQuests _asbp_artemis_frontier_game_instance)
      (if (== _array_element (.RowName (Utilities|Struct|BreakDataTableRowHandle (Variables|Default|GetSecondQuestPrereq))))
        (return true)))
    (return false)
    (else
      (return true))))

(fn Interactwith
  (bind _returnvalue (Components|GetOwner))
  (bind _secondquest (Variables|Default|GetSecondQuest))
  (bind _questdata (Variables|Default|GetQuestData))
  (bind _returnvalue_2 (Utilities|GetDisplayName _returnvalue))
  (bind _asbp_artemis_frontier_game_instance (Utilities|Casting|CastToBP_ArtemisFrontierGameInstance (Game|GetGameInstance)))
  (if (and (not (Default|QueryActiveQuest _asbp_artemis_frontier_game_instance (.rowname _questdata))) (not (.ReturnValue (Default|QueryCompletedQuests _asbp_artemis_frontier_game_instance (.rowname _questdata)))))
    (bind _returnvalue_3 (Utilities|GetDataTableRow "/Game/QuestSystem/EnumsDataTables/QuestData.QuestData" (.rowname (Variables|Default|GetQuestData)))
      (:then
        (if (.AutoAccept (Utilities|Struct|BreakStruct_FQuestDetails _returnvalue_3))
          (bind _asbp_artemis_frontier_game_instance_2 (Utilities|Casting|CastToBP_ArtemisFrontierGameInstance (Game|GetGameInstance)))
          (Default|AddNewQuest _asbp_artemis_frontier_game_instance_2 (.rowname (Variables|Default|GetQuestData)))
          (return (Utilities|GetDisplayName (Components|GetOwner)))
          (elif (Variables|Default|GetRequiresPreRec)
            (bind _newparam (CallFunction|PreRecQuests))
            (if _newparam
              (CallFunction|DisplayQuest :!label _label)
              (return _returnvalue_2))
            (else
              (goto _label))))))
    (else
      (Utilities|IsValid (.datatable _secondquest)
        (:Is%20Valid
          (if (and (not (Default|QueryActiveQuest _asbp_artemis_frontier_game_instance (.rowname _secondquest))) (not (.ReturnValue (Default|QueryCompletedQuests _asbp_artemis_frontier_game_instance (.rowname _secondquest)))))
            (bind _newparam_2 (CallFunction|PreRecQuests2))
            (if _newparam_2
              (CallFunction|DisplayQuest2)
              (return (Utilities|GetDisplayName (Components|GetOwner)))
              (else
                _))))
        (:Is%20Not%20Valid
          _))
      (bind _asbp_artemis_frontier_game_instance_3 (Utilities|Casting|CastToBP_ArtemisFrontierGameInstance (Game|GetGameInstance)))
      (Utilities|IsValid _asbp_artemis_frontier_game_instance_3
        (:Is%20Valid
          (bind _array_element (Default|GetQuestActor _asbp_artemis_frontier_game_instance_3 (.rowname (Variables|Default|GetQuestData))))
          (Utilities|IsValid _array_element
            (:Is%20Valid
              (if (and (Variables|/Game/QuestSystem/Blueprints/Quest_Base.Quest_Base_C|GetIsCompleted? _array_element) (not (Variables|/Game/QuestSystem/Blueprints/Quest_Base.Quest_Base_C|GetIsTurnedIn? _array_element)))
                (return _returnvalue_2)))))))))

(fn QuestGiver
  (return 0))