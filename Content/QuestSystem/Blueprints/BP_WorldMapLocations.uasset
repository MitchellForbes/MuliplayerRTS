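; BP_WorldMapLocations is a world map location trigger that reports quest objectives, shows its name and switches ambient audio.
; When the RTS camera overlaps it, it calls its objective ID, spawns a notifier widget and, for a new sound, crossfades from other locations.
; The game instance holds the current track and playback position, letting audio resume there.
; Tick fades out non-current locations, two specific tracks autoplay on BeginPlay, and finished audio loops.
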(event Custom|CustomEvent_1
  (params (PlayingSoundWave :type Sound%20Wave%20Object%20Reference) (PlaybackPercent :type Float%20%28single-precision%29))
  (bind _duration (Variables|/Script/Engine.SoundBase|GetDuration PlayingSoundWave))
  (bind _returnvalue (* PlaybackPercent _duration))
  (bind _asbp_artemis_frontier_game_instance (Utilities|Casting|CastToBP_ArtemisFrontierGameInstance (Game|GetGameInstance)))
  (Variables|Default|SetCurrentDuration _returnvalue)
  (Default|CurrentPositioninAudio _asbp_artemis_frontier_game_instance _returnvalue))

(event Custom|Completed
  (bind _asbp_artemis_frontier_game_instance (Utilities|Casting|CastToBP_ArtemisFrontierGameInstance (Game|GetGameInstance)))
  (Default|CurrentPositioninAudio _asbp_artemis_frontier_game_instance 0.0)
  (Audio|Components|Audio|Play (Variables|Default|GetAudioComponent) 0.0))

(event Collision|EventActorBeginOverlap
  (params (OtherActor :type Actor%20Object%20Reference))
  (bind _envromentsound (Variables|Default|GetEnvromentSound))
  (bind _audiocomponent (Variables|Default|GetAudioComponent))
  (Utilities|Casting|CastToRTS_Camera OtherActor)
  (bind _asbp_artemis_frontier_game_instance (Utilities|Casting|CastToBP_ArtemisFrontierGameInstance (Game|GetGameInstance)))
  (Default|CallOnObjectiveIDCalled _asbp_artemis_frontier_game_instance (Variables|Default|GetObjectiveID) 1)
  (bind _returnvalue (UserInterface|CreateWidget "/Game/QuestSystem/Widgets/W_LocationNotifier.W_LocationNotifier_C" 0 (Variables|Default|GetLocationName)))
  (UserInterface|Viewport|AddtoViewport _returnvalue 0)
  (bind _asbp_artemis_frontier_game_instance_2 (Utilities|Casting|CastToBP_ArtemisFrontierGameInstance (Game|GetGameInstance)))
  (if (not (== _envromentsound (Variables|/Game/Blueprints/BP_ArtemisFrontierGameInstance.BP_ArtemisFrontierGameInstance_C|GetEnviromentalAudio _asbp_artemis_frontier_game_instance_2)))
    (Audio|Components|Audio|SetSound (Variables|Default|GetAudioComponent) _envromentsound)
    (Variables|Default|SetCurrentDuration (Variables|/Game/Blueprints/BP_ArtemisFrontierGameInstance.BP_ArtemisFrontierGameInstance_C|GetCurrentDuration _asbp_artemis_frontier_game_instance_2))
    (bind _outactors (Actor|GetAllActorsOfClass "BP_WorldMapLocations_C"))
    (for _array_element _outactors
      (bind _asbp_artemis_frontier_game_instance_3 (Utilities|Casting|CastToBP_ArtemisFrontierGameInstance (Game|GetGameInstance)))
      (Variables|Default|SetCurrentDuration (Variables|/Game/Blueprints/BP_ArtemisFrontierGameInstance.BP_ArtemisFrontierGameInstance_C|GetCurrentDuration _asbp_artemis_frontier_game_instance_3))
      (if (Audio|Components|Audio|IsPlaying (Variables|BP_WorldMapLocations_C|GetAudioComponent _array_element))
        (Audio|Components|Audio|FadeOut (Variables|BP_WorldMapLocations_C|GetAudioComponent _array_element) 1.5 0.0 "Linear" :!class /Script/Engine.AudioComponent)))
    (Utilities|FlowControl|RetriggerableDelay 0.75)
    (bind _asbp_artemis_frontier_game_instance_4 (Utilities|Casting|CastToBP_ArtemisFrontierGameInstance (Game|GetGameInstance)))
    (Default|PlayEnviromentalSounds _asbp_artemis_frontier_game_instance_4 (Variables|Default|GetEnvromentSound))
    (Audio|Components|Audio|FadeOut _audiocomponent 0.0 0.0 "Linear" :!class /Script/Engine.AudioComponent)
    (Audio|Components|Audio|FadeIn _audiocomponent 1.5 1.0 (Variables|Default|GetCurrentDuration) "Linear" :!class /Script/Engine.AudioComponent)))

(event EventTick
  (params (DeltaSeconds :type Float%20%28single-precision%29))
  (bind _asbp_artemis_frontier_game_instance (Utilities|Casting|CastToBP_ArtemisFrontierGameInstance (Game|GetGameInstance)))
  (if (not (== (Variables|/Game/Blueprints/BP_ArtemisFrontierGameInstance.BP_ArtemisFrontierGameInstance_C|GetEnviromentalAudio _asbp_artemis_frontier_game_instance) (Variables|Default|GetEnvromentSound)))
    (Audio|Components|Audio|FadeOut (Variables|Default|GetAudioComponent) 1.5 0.0 "Linear" :!class /Script/Engine.AudioComponent)))

(event EventBeginPlay
  (EventDispatchers|BindEventtoOnAudioPlaybackPercent (Variables|Default|GetAudioComponent) (delegate Custom|CustomEvent_1))
  (EventDispatchers|BindEventtoOnAudioFinished (Variables|Default|GetAudioComponent) (delegate Custom|Completed))
  (Audio|Components|Audio|SetSound (Variables|Default|GetAudioComponent) (Variables|Default|GetEnvromentSound))
  (Audio|Components|Audio|FadeOut (Variables|Default|GetAudioComponent) 0.0 0.0 "Linear" :!class /Script/Engine.AudioComponent)
  (bind _asbp_artemis_frontier_game_instance (Utilities|Casting|CastToBP_ArtemisFrontierGameInstance (Game|GetGameInstance)))
  (Variables|Default|SetCurrentDuration (Variables|/Game/Blueprints/BP_ArtemisFrontierGameInstance.BP_ArtemisFrontierGameInstance_C|GetCurrentDuration _asbp_artemis_frontier_game_instance))
  (if (or (== (Variables|Default|GetEnvromentSound) "/Game/Audio/Music/ARTEMIS_-_NEW_THESSALY.ARTEMIS_-_NEW_THESSALY") (== (Variables|Default|GetEnvromentSound) "/Game/Audio/Music/ARTEMIS_-_MENU_OUTPOST.ARTEMIS_-_MENU_OUTPOST"))
    (bind _asbp_artemis_frontier_game_instance_2 (Utilities|Casting|CastToBP_ArtemisFrontierGameInstance (Game|GetGameInstance)))
    (Default|PlayEnviromentalSounds _asbp_artemis_frontier_game_instance_2 (Variables|Default|GetEnvromentSound))
    (Audio|Components|Audio|Play (Variables|Default|GetAudioComponent) (Variables|Default|GetCurrentDuration))))

(fn ConstructionScript)