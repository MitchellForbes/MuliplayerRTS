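; Quest_Base is a quest Actor that tracks objective progress for the current stage of a quest.
; On BeginPlay it loads its QuestID row from the QuestData table and resets a per-objective counter map for that stage.
; It also binds to the player character's objective-ID event, with OnObjectiveIdHeard incrementing matching counters and ignoring unknown IDs.
; No stage advancement or completion check is implemented here.
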(event EventBeginPlay
  (CallFunction|GetQuestDetails)
  (EventDispatchers|BindEventtoOnObjectiveIDCalled (CallFunction|GetMyPlayerCharacter) (EventDispatchers|CreateEvent :!event OnObjectiveIdHeard)))

(event Collision|EventActorBeginOverlap
  (params (OtherActor :type Actor%20Object%20Reference)))

(event EventTick
  (params (DeltaSeconds :type Float%20%28single-precision%29)))

(fn ConstructionScript)

(fn OnObjectiveIdHeard
  (params (ObjectiveID :type String))
  (bind _currentobjectiveprogress (Variables|Default|GetCurrentObjectiveProgress))
  (bind (_value _returnvalue) (Utilities|Map|Find _currentobjectiveprogress ObjectiveID))
  (if _returnvalue
    (Utilities|Map|Add (Variables|Default|GetCurrentObjectiveProgress) ObjectiveID (+ _value 1))
    (return)
    (else
      (return))))

(fn GetQuestDetails
  (bind _returnvalue (Utilities|GetDataTableRow "/Game/QuestSystem/EnumsDataTables/QuestData.QuestData" (Variables|Default|GetQuestID))
    (:then
      (bind _output_get (Variables|Default|SetQuestDetails _returnvalue))
      (bind _output_get_2 (Variables|Default|SetCurrentStageDetails (Utilities|Array|Get(acopy) (.Stages (Utilities|Struct|BreakStruct_FQuestDetails _output_get)) (Variables|Default|GetCurrentStage))))
      (Utilities|Map|Clear (Variables|Default|GetCurrentObjectiveProgress))
      (for _array_element (.Objectives (Utilities|Struct|BreakStruct_FStageDetails _output_get_2))
        (Utilities|Map|Add (Variables|Default|GetCurrentObjectiveProgress) (.ObjectiveID (Utilities|Struct|BreakStruct_FObjectiveDetails _array_element)) 0)))))