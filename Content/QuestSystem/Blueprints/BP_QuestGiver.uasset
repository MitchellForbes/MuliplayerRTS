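; BP_QuestGiver hands a quest, identified by its QuestData row name, to the player through a GiveQuest event.
; If its quest log reference is invalid, it adds a BPCQuestLog component to the first player controller and stores it.
; When that log does not report the quest as active, it asks BP_ArtemisFrontierGameInstance to add the new quest.
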(event Custom|GiveQuest
  (Utilities|IsValid (Variables|Default|GetBPCQuestLog)
    (:Is%20Valid
      _)
    (:Is%20Not%20Valid
      (bind _returnvalue (AddComponent|AddBPCQuestLogComponent (Game|GetPlayerController 0)))
      (Variables|Default|SetBPCQuestLog _returnvalue)))
  (if (not (Default|QueryActiveQuest (Variables|Default|GetBPCQuestLog) (.rowname (Variables|Default|GetQuestData))))
    (bind _asbp_artemis_frontier_game_instance (Utilities|Casting|CastToBP_ArtemisFrontierGameInstance (Game|GetGameInstance)))
    (Default|AddNewQuest _asbp_artemis_frontier_game_instance (.rowname (Variables|Default|GetQuestData)))))

(fn ConstructionScript)