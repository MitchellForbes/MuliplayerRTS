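; BP_Clouds is a cloud actor that drifts through the level on a repeating path.
; On BeginPlay it stores its starting location.
; Each Tick it moves by Velocity without delta-time scaling, so drift speed depends on frame rate.
; Once its distance from the start exceeds MaxDistance, it snaps back to the starting location, looping the motion.
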(event EventBeginPlay
  (Variables|Default|SetStarting%20Location (Transformation|GetActorLocation)))

(event EventTick
  (params (DeltaSeconds :type Float%20%28single-precision%29))
  (Transformation|SetActorLocation (+ (Transformation|GetActorLocation) (Variables|Default|GetVelocity)) false false)
  (if (> (Math|Vector|Distance(Vector) (Variables|Default|GetStarting%20Location) (Transformation|GetActorLocation)) (Variables|Default|GetMaxDistance))
    (Transformation|SetActorLocation (Variables|Default|GetStarting%20Location) false false)))

(fn ConstructionScript)